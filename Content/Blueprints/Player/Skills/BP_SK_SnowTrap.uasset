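; Player skill Blueprint for the Snow Trap, which places a skill object at the mouse or finger position.
; Skill start spawns a landing marker at the character's transform and passes it the player controller.
; Skill end consumes mana, spawns the skill object at the pointer position with the character as owner and instigator, then destroys the marker.
; Skill tick only calls the parent, and ModifyManaValues is empty.
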(event EventBeginPlay
  (|CallParentFunction) ; This node is disabled and will not be called.\nDrag off pins to build functionality.
)

(event EventTick
  (params (DeltaSeconds :type Float%20%28single-precision%29))
  (|CallParentFunction DeltaSeconds) ; This node is disabled and will not be called.\nDrag off pins to build functionality.
)

(fn OnSkillStart
  (bind _playercontroller (Variables|Default|GetPlayerController))
  (bind _playercharacter (Variables|/Game/Blueprints/Player/BP_PlayerController.BP_PlayerController_C|GetPlayerCharacter _playercontroller))
  (|CallParentFunction)
  (bind _returnvalue (Game|SpawnActorfromClass (Variables|Default|GetLandingMarkerClass) (Transformation|GetActorTransform _playercharacter) "AlwaysSpawn" _playercontroller _playercontroller _playercharacter))
  (Variables|Default|SetLandingMarkerObject _returnvalue))

(fn OnSkillTick
  (|CallParentFunction))

(fn OnSkillEnd
  (bind _playercontroller (Variables|Default|GetPlayerController))
  (bind _playercharacter (Variables|/Game/Blueprints/Player/BP_PlayerController.BP_PlayerController_C|GetPlayerCharacter _playercontroller))
  (|CallParentFunction)
  (CallFunction|ConsumeMana)
  (bind _convertedposition (Default|GetMouseorFingerPosition _playercontroller))
  (Game|SpawnActorfromClass (Variables|Default|GetSkillObjectClass) (Math|Transform|MakeTransform _convertedposition "0, 0, 0" "1.000000,1.000000,1.000000") "AlwaysSpawn" _playercharacter _playercharacter)
  (Actor|DestroyActor (Variables|Default|GetLandingMarkerObject)))

(fn ModifyManaValues
  (params (Increase :type Boolean) (Amount :type Float%20%28double-precision%29)))