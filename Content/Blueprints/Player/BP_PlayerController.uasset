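; Player controller that spawns and possesses the game instance's chosen hero, turning pointer input into hero taps and lane swipe attacks.
; Press and release raycasts from the hero camera, using touch deprojected onto the hero's plane (PC branch yields zero vectors), identify the hero or tagged lanes.
; Taps grant a timed attack-speed boost; swipes from the hero attack along the lane's forward vector.
; Skill button and enemy-kill mana calls forward to the hero.
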(event Custom|OnAttackSpeedIncrease
  (Default|ModifyAttackSpeed (Variables|Default|GetPlayerCharacter) false))

(event Custom|OnHeroClick
  (Default|OnHeroClicked (Variables|Default|GetPlayerCharacter)))

(event Custom|OnHeroSwipe
  (params (Lane :type Actor%20Object%20Reference))
  (if (Variables|/Game/Blueprints/Characters/Frontline/Hero/BP_HeroBase.BP_HeroBase_C|GetbIsTapped (Variables|Default|GetPlayerCharacter))
    (bind _swipedir (CallFunction|GetSwipeDirection Lane))
    (Default|SpawnSwipeAttack (Variables|Default|GetPlayerCharacter) _swipedir)
    (else
      (CallFunction|OnHeroTapped))))

(event Custom|OnHeroTapped
  (Default|ModifyAttackSpeed (Variables|Default|GetPlayerCharacter) true)
  (Utilities|FlowControl|Sequence
    (:then_0
      (if (Utilities|Time|IsValidTimerHandle (Variables|Default|GetAttackSpeedTimer))
        (Utilities|Time|ClearandInvalidateTimerbyHandle (Variables|Default|GetAttackSpeedTimer))))
    (:then_1
      (bind _returnvalue (Utilities|Time|SetTimerbyEvent (delegate Custom|OnAttackSpeedIncrease) (Variables|Default|GetIncreaseAttackSpeedDuration)))
      (Variables|Default|SetAttackSpeedTimer _returnvalue))))

(event EventBeginPlay
  (Utilities|FlowControl|Sequence
    (:then_0
      (bind _herocharacterpicked (Default|GetPlayerCharacter (CallFunction|GetFrontlineGameInstance)))
      (bind _returnvalue (Game|SpawnActorfromClass _herocharacterpicked (Transformation|GetActorTransform (Pawn|GetControlledPawn)) "AlwaysSpawn" "SelectDefaultAtRuntime" 0 0))
      (bind _output_get (Variables|Default|SetPlayerCharacter _returnvalue))
      (Actor|DestroyActor (Pawn|GetControlledPawn))
      (Pawn|Possess _output_get))
    (:then_1
      (Input|AddMappingContext (PlayerController|LocalPlayerSubsystems|GetEnhancedInputLocalPlayerSubsystem) "/Game/Input/IMC_Mobile.IMC_Mobile" 1 "(bIgnoreAllPressedKeysUntilRelease=True,bForceImmediately=False,bNotifyUserSettings=False)"))
    (:then_2
      (Input|SetInputModeGameandUI self 0 "LockOnCapture" false false))))

(event Input|ActionEvents|InputActionInteractx
  (params (Key :type Key%20Structure :default "None"))
  (bind _playercharacter (Variables|Default|GetPlayerCharacter))
  (:Pressed
    (bind _hitactor (CallFunction|RaycastfromCamera true))
    (Utilities|IsValid _hitactor
      (:Is%20Valid
        (if (== _hitactor _playercharacter)
          (CallFunction|OnHeroClick)
          (else
            (Variables|/Game/Blueprints/Characters/Frontline/Hero/BP_HeroBase.BP_HeroBase_C|SetbIsTapped _playercharacter false :!label _label))))
      (:Is%20Not%20Valid
        (goto _label))))
  (:Released
    (bind _hitactor_2 (CallFunction|RaycastfromCamera false))
    (Utilities|IsValid _hitactor_2
      (:Is%20Valid
        (if (== _hitactor_2 (Variables|Default|GetPlayerCharacter))
          (CallFunction|OnHeroTapped)
          (elif (Actor|ActorHasTag _hitactor_2 "LevelLane")
            (CallFunction|OnHeroSwipe _hitactor_2)
            (Variables|/Game/Blueprints/Characters/Frontline/Hero/BP_HeroBase.BP_HeroBase_C|SetbIsTapped (Variables|Default|GetPlayerCharacter) false)
            (else
              (CallFunction|OnHeroTapped :!label _label_2)))))
      (:Is%20Not%20Valid
        (goto _label_2)))))

(fn ConstructionScript)

(fn ConvertSwipeDirection
  (params (Direction :type Vector%202D%20Structure))
  (bind (_x _y) (Math|Vector2D|BreakVector2D Direction))
  (Utilities|FlowControl|Sequence
    (:then_0
      (bind _outactors (Actor|GetAllActorsOfClass "/Game/Blueprints/Managers/SpawnPoint.SpawnPoint_C"))
      (LocalVariables|SetSpawnPoints _outactors))
    (:then_1
      (LocalVariables|SetTopSwipe (< _y 0.0)))
    (:then_2
      (LocalVariables|SetRightSwipe (> _x 0.0)))
    (:then_3
      (LocalVariables|SetLeftSwipe (< _x 0.0)))
    (:then_4
      (if (LocalVariables|GetLeftSwipe)
        (bind _array_element (Utilities|Array|ForEachLoopwithBreak (LocalVariables|GetSpawnPoints) :!label _label)
          (:LoopBody
            (if (Utilities|Enum|Equal(Enum) (Utilities|GetDisplayName _array_element) "LeftSP")
              (LocalVariables|SetChosenPoint (Transformation|GetActorLocation _array_element))
              (goto _label Break))))
        (elif (LocalVariables|GetRightSwipe)
          (bind _array_element_2 (Utilities|Array|ForEachLoopwithBreak (LocalVariables|GetSpawnPoints) :!label _label_2)
            (:LoopBody
              (if (Utilities|Enum|Equal(Enum) (Utilities|GetDisplayName _array_element_2) "RightSP")
                (LocalVariables|SetChosenPoint (Transformation|GetActorLocation _array_element_2))
                (goto _label_2 Break))))
          (elif (LocalVariables|GetTopSwipe)
            (bind _array_element_3 (Utilities|Array|ForEachLoopwithBreak (LocalVariables|GetSpawnPoints) :!label _label_3)
              (:LoopBody
                (if (Utilities|Enum|Equal(Enum) (Utilities|GetDisplayName _array_element_3) "TopSP")
                  (LocalVariables|SetChosenPoint (Transformation|GetActorLocation _array_element_3))
                  (goto _label_3 Break))))))))
    (:then_5
      (return (Math|Conversions|ToVector2D(Vector) (Class|KismetMathLibrary|VectorNormal2D (- (LocalVariables|GetChosenPoint) (Transformation|GetActorLocation (Variables|Default|GetPlayerCharacter))) 0.0001))))))

(fn OnEnemyKilled
  (params (ManaEarned :type Integer))
  (Default|OnEnemyKilled (Variables|Default|GetPlayerCharacter) ManaEarned))

(fn OnSkillButtonStart
  (params (SkillID :type Integer))
  (Default|OnSkillStart (Variables|Default|GetPlayerCharacter) SkillID))

(fn OnSkillButtonRelease
  (params (SkillID :type Integer))
  (Default|OnSkillEnd (Variables|Default|GetPlayerCharacter) SkillID))

(fn CheckSkillAvailable
  (params (SkillID :type Integer))
  (bind _playercharacter (Variables|Default|GetPlayerCharacter))
  (Utilities|IsValid _playercharacter
    (:Is%20Valid
      (bind _available (Default|CheckSkillAvailable _playercharacter SkillID))
      (return _available))))

(fn RaycastfromCamera
  (params (Pressed :type Boolean))
  (bind _playercharacter (Variables|Default|GetPlayerCharacter))
  (bind _camera (Variables|/Game/Blueprints/Characters/Frontline/Hero/BP_HeroBase.BP_HeroBase_C|GetCamera _playercharacter))
  (bind _returnvalue (Transformation|GetWorldLocation _camera))
  (Utilities|FlowControl|Sequence
    (:then_0
      (if Pressed
        (bind _output_get (LocalVariables|SetTraceColor (Class|KismetMathLibrary|LinearColorBlue)))
        (else
          (bind _output_get_2 (LocalVariables|SetTraceColor (Class|KismetMathLibrary|LinearColorRed))))))
    (:then_1
      (bind (_outhit _returnvalue_2) (Collision|LineTraceByChannel _returnvalue (* (Math|Vector|Normalize (- (.WorldLoc (CallFunction|GetInteractPosition)) _returnvalue)) 5e+04) "TraceTypeQuery3" false 0 "ForDuration" true (LocalVariables|GetTraceColor) "(R=0.000000,G=1.000000,B=0.000000,A=1.000000)" 1.0))
      (if _returnvalue_2
        (return (.HitActor (Collision|BreakHitResult _outhit)))))))

(fn GetInteractPosition
  (bind (_locationx _locationy) (Class|PlayerController|GetInputTouchState "Touch1"))
  (bind (_worldlocation _worlddirection) (Class|PlayerController|DeprojectScreenPositiontoWorld _locationx _locationy))
  (Utilities|FlowControl|Sequence
    (:then_0
      (switch Utilities|FlowControl|Switch|SwitchonEnum_Platforms (Default|GetCurrentPlatform (CallFunction|GetFrontlineGameInstance))
        (:NewEnumerator0
          (bind _returnvalue (Class|WidgetLayoutLibrary|GetMousePositiononViewport))
          (LocalVariables|SetWorldLocation "0, 0, 0")
          (LocalVariables|SetWorldDirection "0, 0, 0"))
        (:NewEnumerator1
          (LocalVariables|SetWorldLocation _worldlocation)
          (LocalVariables|SetWorldDirection _worlddirection))))
    (:then_1
      (return (.Intersection (Class|KismetMathLibrary|LinePlaneIntersectionOriginNormal (LocalVariables|GetWorldLocation) (+ (LocalVariables|GetWorldLocation) (* (LocalVariables|GetWorldDirection) 5e+06)) (Transformation|GetActorLocation (Variables|Default|GetPlayerCharacter)) "0, 0,1.000000")) (LocalVariables|GetWorldDirection)))))

(fn GetSwipeDirection
  (params (Lane :type Actor%20Object%20Reference))
  (return (Math|Conversions|ToVector2D(Vector) (Class|KismetMathLibrary|VectorNormal2D (Math|Rotator|GetRotationXVector (Transformation|GetActorRotation Lane)) 0.0001))))