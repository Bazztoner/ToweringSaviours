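; Slash attack skill Blueprint that extends a parent skill's start and end hooks to place an effect through a landing marker.
; On start it spawns the landing marker at the player character's transform, passing in the player controller.
; On end it consumes mana, spawns the skill object at the marker's transform with the character as owner and instigator, then destroys the marker.
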(event EventBeginPlay
  (|CallParentFunction))

(event EventTick
  (params (DeltaSeconds :type Float%20%28single-precision%29))
  (|CallParentFunction DeltaSeconds) ; This node is disabled and will not be called.\nDrag off pins to build functionality.
)

(fn OnSkillStart
  (bind _playercontroller (Variables|Default|GetPlayerController))
  (bind _playercharacter (Variables|/Game/Blueprints/Player/BP_PlayerController.BP_PlayerController_C|GetPlayerCharacter _playercontroller))
  (|CallParentFunction)
  (bind _returnvalue (Game|SpawnActorfromClass (Variables|Default|GetLandingMarkerClass) (Transformation|GetActorTransform _playercharacter) "AlwaysSpawn" "SelectDefaultAtRuntime" _playercontroller _playercontroller _playercharacter))
  (Variables|Default|SetLandingMarkerObject _returnvalue))

(fn OnSkillEnd
  (bind _playercontroller (Variables|Default|GetPlayerController))
  (bind _playercharacter (Variables|/Game/Blueprints/Player/BP_PlayerController.BP_PlayerController_C|GetPlayerCharacter _playercontroller))
  (|CallParentFunction)
  (CallFunction|ConsumeMana)
  (Game|SpawnActorfromClass (Variables|Default|GetSkillObjectClass) (Transformation|GetActorTransform (Variables|Default|GetLandingMarkerObject)) "AlwaysSpawn" "SelectDefaultAtRuntime" _playercharacter 75.0 0.5 _playercharacter)
  (Actor|DestroyActor (Variables|Default|GetLandingMarkerObject)))