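; Player shotgun skill that previews a cone and then spawns a pellet attack.
; On skill start, it rotates the projectile spawn point's forward vector by plus and minus HalfAngle around up and passes both edge directions to a landing marker spawned at the character.
; On skill end, it consumes mana, spawns the skill object at the marker's transform with pellet, damage and angle settings, then destroys the marker.
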(event EventBeginPlay
  (|CallParentFunction))

(event EventTick
  (params (DeltaSeconds :type Float%20%28single-precision%29))
  (|CallParentFunction DeltaSeconds) ; This node is disabled and will not be called.\nDrag off pins to build functionality.
)

(fn OnSkillStart
  (bind _playercontroller (Variables|Default|GetPlayerController))
  (bind _playercharacter (Variables|/Game/Blueprints/Player/BP_PlayerController.BP_PlayerController_C|GetPlayerCharacter _playercontroller))
  (Utilities|FlowControl|Sequence
    (:then_0
      (|CallParentFunction))
    (:then_1
      (bind (_leftpoint _rightpoint) (CallFunction|GetConePoints (Variables|Default|GetHalfAngle)))
      (LocalVariables|SetLeftPoint _leftpoint)
      (LocalVariables|SetRightPoint _rightpoint))
    (:then_2
      (bind _returnvalue (Game|SpawnActorfromClass (Variables|Default|GetLandingMarkerClass) (Transformation|GetActorTransform _playercharacter) "AlwaysSpawn" "SelectDefaultAtRuntime" _playercontroller (LocalVariables|GetLeftPoint) (LocalVariables|GetRightPoint) "0.000000,0.000000,0.000000" 1.5e+03 _playercontroller _playercharacter))
      (Variables|Default|SetLandingMarkerObject _returnvalue))))

(fn OnSkillEnd
  (bind _playercontroller (Variables|Default|GetPlayerController))
  (|CallParentFunction)
  (CallFunction|ConsumeMana)
  (Game|SpawnActorfromClass (Variables|Default|GetSkillObjectClass) (Transformation|GetActorTransform (Variables|Default|GetLandingMarkerObject)) "AlwaysSpawn" "SelectDefaultAtRuntime" _playercontroller (Variables|Default|GetPellets) (Variables|Default|GetDamage) (Variables|Default|GetHalfAngle) (Variables|/Game/Blueprints/Player/BP_PlayerController.BP_PlayerController_C|GetPlayerCharacter _playercontroller))
  (Actor|DestroyActor (Variables|Default|GetLandingMarkerObject)))

(fn GetConePoints
  (params (RotationAngle :type Float%20%28double-precision%29))
  (return (Math|Vector|RotateVectorAroundAxis (Math|Vector|GetForwardVector (Variables|/Game/Blueprints/Characters/Frontline/Hero/BP_HeroBase.BP_HeroBase_C|GetProjSpawnPos (Variables|/Game/Blueprints/Player/BP_PlayerController.BP_PlayerController_C|GetPlayerCharacter (Variables|Default|GetPlayerController)))) (* RotationAngle -1.0) (Math|Vector|VectorUp)) (Math|Vector|RotateVectorAroundAxis (Math|Vector|GetForwardVector (Variables|/Game/Blueprints/Characters/Frontline/Hero/BP_HeroBase.BP_HeroBase_C|GetProjSpawnPos (Variables|/Game/Blueprints/Player/BP_PlayerController.BP_PlayerController_C|GetPlayerCharacter (Variables|Default|GetPlayerController)))) RotationAngle (Math|Vector|VectorUp))))