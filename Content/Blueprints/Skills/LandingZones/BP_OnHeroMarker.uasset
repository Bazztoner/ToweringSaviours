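; BP_OnHeroMarker is a skill landing-zone marker that stays on the player's hero while tracking the aim direction.
; On BeginPlay it caches the player character's ProjSpawnPos component.
; Each Tick it sets its yaw from the flattened vector between the controller's interact position and that component, so its X axis points away from the interact point.
; It then snaps its location to the component's world position.
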(event EventBeginPlay
  (|CallParentFunction)
  (Variables|Default|SetLocationTransform (Variables|/Game/Blueprints/Characters/Frontline/Hero/BP_HeroBase.BP_HeroBase_C|GetProjSpawnPos (Variables|/Game/Blueprints/Player/BP_PlayerController.BP_PlayerController_C|GetPlayerCharacter (Variables|Default|GetPlayerController)))))

(event Collision|EventActorBeginOverlap
  (params (OtherActor :type Actor%20Object%20Reference))
  (|CallParentFunction OtherActor) ; This node is disabled and will not be called.\nDrag off pins to build functionality.
)

(event EventTick
  (params (DeltaSeconds :type Float%20%28single-precision%29))
  (|CallParentFunction DeltaSeconds)
  (CallFunction|SetRotation)
  (CallFunction|ForcePosition))

(fn ConstructionScript
  (|CallParentFunction))

(fn ForcePosition
  (Transformation|SetActorLocation (Transformation|GetWorldLocation (Variables|Default|GetLocationTransform)) false false))

(fn SetRotation
  (Transformation|SetActorRotation (Math|Conversions|RotationFromXVector (Class|KismetMathLibrary|VectorNormal2D (- (Transformation|GetWorldLocation (Variables|Default|GetLocationTransform)) (.WorldLoc (Default|GetInteractPosition (Variables|Default|GetPlayerController)))) 0.0001))))