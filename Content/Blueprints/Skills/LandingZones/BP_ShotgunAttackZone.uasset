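; BP_ShotgunAttackZone is a skill landing zone that displays the cone-shaped area of a shotgun attack.
; On BeginPlay, after the parent logic, it scales its left and right points by the cone length.
; CreateCone then builds a single-triangle procedural mesh from those points and the origin, and applies the shotgun zone material.
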(event EventBeginPlay
  (|CallParentFunction)
  (CallFunction|CreateCone))

(fn ConstructionScript
  (|CallParentFunction))

(fn CreateCone
  (bind _proceduralcone (Variables|Default|GetProceduralCone))
  (bind _conelength (Variables|Default|GetConeLength))
  (Utilities|FlowControl|Sequence
    (:then_0
      (Variables|Default|SetLeftPoint (* (Variables|Default|GetLeftPoint) _conelength)))
    (:then_1
      (Variables|Default|SetRightPoint (* (Variables|Default|GetRightPoint) _conelength)))
    (:then_2
      (Class|ProceduralMeshComponent|CreateMeshSectionLinearColor _proceduralcone 0 (Utilities|Array|MakeArray (Variables|Default|GetLeftPoint) (Variables|Default|GetOrigin) (Variables|Default|GetRightPoint)) (Utilities|Array|MakeArray 0 1 2) 0 0 0 0 0 0 0 false false)
      (Rendering|Material|SetMaterial _proceduralcone 0 "/Game/Art/Materials/Skills/M_ShotgunZone.M_ShotgunZone"))))