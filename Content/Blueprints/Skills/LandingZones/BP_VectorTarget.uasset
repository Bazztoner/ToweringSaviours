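; BP_VectorTarget is a skill landing-zone actor that orients itself relative to the player character's projectile spawn point.
; Every Tick, SetRotation points its X axis along the direction from ProjSpawnPos to the actor, so it faces away from the spawn point.
; SetSplinePosition would set the SplineMesh end to the spawn point's XY offset from the actor, but its call in the event graph is unconnected.
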(event EventBeginPlay
  (|CallParentFunction) ; This node is disabled and will not be called.\nDrag off pins to build functionality.
)

(event Collision|EventActorBeginOverlap
  (params (OtherActor :type Actor%20Object%20Reference))
  (|CallParentFunction OtherActor) ; This node is disabled and will not be called.\nDrag off pins to build functionality.
)

(event EventTick
  (params (DeltaSeconds :type Float%20%28single-precision%29))
  (|CallParentFunction DeltaSeconds)
  (CallFunction|SetRotation))

(fn ConstructionScript
  (|CallParentFunction))

(fn SetRotation
  (Transformation|SetActorRotation (Math|Conversions|RotationFromXVector (Math|Vector|Normalize (- (Transformation|GetActorLocation) (Transformation|GetWorldLocation (Variables|/Game/Blueprints/Characters/Frontline/Hero/BP_HeroBase.BP_HeroBase_C|GetProjSpawnPos (Variables|/Game/Blueprints/Player/BP_PlayerController.BP_PlayerController_C|GetPlayerCharacter (Variables|Default|GetPlayerController)))))))))

(fn SetSplinePosition
  (bind _returnvalue (Transformation|GetActorLocation))
  (bind _playercontroller (Variables|Default|GetPlayerController))
  (bind _playercharacter (Variables|/Game/Blueprints/Player/BP_PlayerController.BP_PlayerController_C|GetPlayerCharacter _playercontroller))
  (bind _projspawnpos (Variables|/Game/Blueprints/Characters/Frontline/Hero/BP_HeroBase.BP_HeroBase_C|GetProjSpawnPos _playercharacter))
  (bind _returnvalue_2 (Transformation|GetWorldLocation _projspawnpos))
  (bind _returnvalue_3 (Math|Vector|MakeVector (.x _returnvalue_2) (.y _returnvalue_2) 0.0))
  (bind _returnvalue_4 (- _returnvalue_3 _returnvalue))
  (SplineMesh|SetEndPosition (Variables|Default|GetSplineMesh) (Math|Vector|MakeVector (.x _returnvalue_4) (.y _returnvalue_4) 0.0) true))