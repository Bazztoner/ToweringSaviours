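; BP_BarbedWireLandingZone is a landing zone Blueprint, apparently the placement marker for a barbed wire skill, that aligns itself to the level lane beneath it.
; Each Tick runs the parent logic, then line traces 5000 units straight down on the Visibility channel.
; When the hit actor carries the LevelLane tag, the zone copies that actor's rotation.
; The construction script only calls its parent.
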(event EventTick
  (params (DeltaSeconds :type Float%20%28single-precision%29))
  (bind _returnvalue (Transformation|GetActorLocation))
  (bind (_x _y _z) (Math|Vector|BreakVector _returnvalue))
  (|CallParentFunction DeltaSeconds)
  (bind (_outhit _returnvalue_2) (Collision|LineTraceByChannel _returnvalue (Math|Vector|MakeVector _x _y (- _z 5e+03)) "TraceTypeQuery1" false 0 "None"))
  (if _returnvalue_2
    (if (Actor|ActorHasTag (.HitActor (Collision|BreakHitResult _outhit)) "LevelLane")
      (Transformation|SetActorRotation (Transformation|GetActorRotation (.HitActor (Collision|BreakHitResult _outhit)))))))

(fn ConstructionScript
  (|CallParentFunction))