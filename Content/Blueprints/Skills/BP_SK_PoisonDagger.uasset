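; BP_SK_PoisonDagger is a player skill that launches a poison dagger toward the mouse or finger position.
; On skill start it spawns a landing marker at the player character.
; On skill end it aims from the character's projectile spawn point using the 2D-normalized direction to the cursor, consumes mana, spawns the skill object there and destroys the marker.
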(event EventBeginPlay
  (|CallParentFunction) ; This node is disabled and will not be called.\nDrag off pins to build functionality.
)

(event EventTick
  (params (DeltaSeconds :type Float%20%28single-precision%29))
  (|CallParentFunction DeltaSeconds) ; This node is disabled and will not be called.\nDrag off pins to build functionality.
)

(fn OnSkillStart
  (bind _playercontroller (Variables|Default|GetPlayerController))
  (bind _playercharacter (Variables|/Game/Blueprints/Player/BP_PlayerController.BP_PlayerController_C|GetPlayerCharacter _playercontroller))
  (|CallParentFunction)
  (bind _returnvalue (Game|SpawnActorfromClass (Variables|Default|GetLandingMarkerClass) (Transformation|GetActorTransform _playercharacter) "AlwaysSpawn" "SelectDefaultAtRuntime" _playercontroller _playercontroller _playercharacter))
  (Variables|Default|SetLandingMarkerObject _returnvalue))

(fn OnSkillEnd
  (bind _playercontroller (Variables|Default|GetPlayerController))
  (bind _playercontroller_2 (Variables|Default|GetPlayerController))
  (bind _playercharacter (Variables|/Game/Blueprints/Player/BP_PlayerController.BP_PlayerController_C|GetPlayerCharacter _playercontroller))
  (bind _playercharacter_2 (Variables|/Game/Blueprints/Player/BP_PlayerController.BP_PlayerController_C|GetPlayerCharacter _playercontroller_2))
  (bind _projspawnpos (Variables|/Game/Blueprints/Characters/Frontline/Hero/BP_HeroBase.BP_HeroBase_C|GetProjSpawnPos _playercharacter))
  (bind _returnvalue (Transformation|GetWorldLocation _projspawnpos))
  (|CallParentFunction)
  (Utilities|FlowControl|Sequence
    (:then_0
      (bind _convertedposition (Default|GetMouseorFingerPosition _playercontroller))
      (LocalVariables|SetProjectileDirection (Math|Conversions|RotationFromXVector (Class|KismetMathLibrary|VectorNormal2D (- _convertedposition _returnvalue) 0.0001)))
      (LocalVariables|SetProjectileSpawnPos _returnvalue))
    (:then_1
      (CallFunction|ConsumeMana)
      (Game|SpawnActorfromClass (Variables|Default|GetSkillObjectClass) (Math|Transform|MakeTransform (LocalVariables|GetProjectileSpawnPos) (LocalVariables|GetProjectileDirection) "1.000000,1.000000,1.000000") "AlwaysSpawn" "SelectDefaultAtRuntime" _playercharacter_2 _playercharacter_2)
      (Actor|DestroyActor (Variables|Default|GetLandingMarkerObject)))))