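; Base Frontline enemy character that chases the player and deals damage once in range, dying as it attacks.
; A screen-projected HP bar follows it, appearing when damaged.
; Knockback briefly interrupts pursuit and slow events scale walk speed, while a looping timer kills enemies stuck near spawn.
; Death reports to BP_WaveManager, spawning one if absent, and spawns explosion effects or flags IsDead, depending on mesh visibility and killer.
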(event Custom|OnAttack
  (bind _returnvalue (Utilities|Time|SetTimerbyEvent (delegate Custom|EnableAttack) (Variables|Default|GetAttackCooldown)))
  (Variables|Default|SetAttackCooldownTimer _returnvalue))

(event Custom|EnableAttack
  (Variables|Default|SetbCanAttack true))

(event Custom|ApplyKnockback
  (params (ForceVector :type Vector))
  (AI|Navigation|StopMovement (Pawn|GetController))
  (Utilities|FlowControl|DelayUntilNextTick)
  (Physics|AddImpulse (Variables|Character|GetCharacterMovement) ForceVector true)
  (Utilities|FlowControl|RetriggerableDelay (Variables|Default|GetKnockbackTimeout))
  (AI|Navigation|SimpleMovetoActor (Pawn|GetController) (Variables|Default|GetPlayerActor)))

(event Custom|CheckCanMove
  (if (and (<= (Math|Vector|Distance2D(Vector) (Transformation|GetActorLocation) (Variables|Default|GetSpawnPos)) 5e+02) (< (Math|Vector|VectorLengthSquared (Transformation|GetVelocity)) 1.0))
    (Development|PrintString "I'M STUCK :(")
    (CallFunction|Die)))

(event Custom|OnSlowApplied
  (params (SlowMultiplier :type Float%20%28double-precision%29) (isSlowed :type Boolean))
  (CallFunction|ApplySlow SlowMultiplier isSlowed))

(event Custom|Ev_DelayedDeath
  (Utilities|FlowControl|Delay 1.0)
  (Actor|DestroyActor))

(event EventBeginPlay
  (Variables|Default|SetSpawnPos (Transformation|GetActorLocation))
  (Utilities|Time|SetTimerbyEvent (delegate Custom|CheckCanMove) 3e+01 true)
  (|CallParentFunction)
  (bind _output_get (Variables|Default|SetPlayerActor (Variables|/Game/Blueprints/Player/BP_PlayerController.BP_PlayerController_C|GetPlayerCharacter (CallFunction|GetFrontlinePlayerController))))
  (AI|Navigation|SimpleMovetoActor (Pawn|GetController) _output_get)
  (Variables|Default|SetDefaultMovementSpeed (Variables|/Script/Engine.CharacterMovementComponent|GetMaxWalkSpeed (Variables|Character|GetCharacterMovement)))
  (bind _returnvalue (UserInterface|CreateWidget "/Game/Blueprints/Widgets/Frontline/HUD_EnemyHPBar.HUD_EnemyHPBar_C" 0 self))
  (bind _output_get_2 (Variables|Default|SetHPBar _returnvalue))
  (UserInterface|Viewport|AddtoViewport _output_get_2 1)
  (Widget|SetVisibility (Variables|Default|GetHPBar) "Collapsed"))

(event EventTick
  (params (DeltaSeconds :type Float%20%28single-precision%29))
  (Utilities|FlowControl|Sequence
    (:then_0
      (Class|UserWidget|SetPositioninViewport (Variables|Default|GetHPBar) (.ScreenPosition (Class|GameplayStatics|ProjectWorldtoScreen (CallFunction|GetFrontlinePlayerController) (Transformation|GetActorLocation) false)) true))
    (:then_1
      (bind _attackavailable (CallFunction|CheckAttackAvailable))
      (if _attackavailable
        (CallFunction|Attack)))))

(event Collision|EventActorBeginOverlap
  (params (OtherActor :type Actor%20Object%20Reference)))

(event Collision|EventActorEndOverlap
  (params (OtherActor :type Actor%20Object%20Reference)))

(fn ConstructionScript
  (|CallParentFunction))

(fn Attack
  (Variables|Default|SetbCanAttack false)
  (Game|Damage|ApplyDamage (Variables|Default|GetPlayerActor) (Variables|Default|GetAttackDamage) 0 0)
  (CallFunction|OnAttack)
  (Variables|Default|SetbKilledByPlayer false)
  ;[1 0.07802 0.9681] Destroy after attack
  (CallFunction|Die))

(fn Die
  (bind _self self)
  (bind _hpbar (Variables|Default|GetHPBar))
  (bind _returnvalue (Pawn|GetController _self))
  (Utilities|FlowControl|Sequence
    (:then_0
      (Collision|SetCollisionEnabled (Variables|Default|GetCapsuleComponent) "NoCollision")
      (Physics|SetEnableGravity (Variables|Default|GetCapsuleComponent) false))
    (:then_1
      (Utilities|IsValid (Variables|Default|GetWaveManager)
        (:Is%20Not%20Valid
          (bind _returnvalue_2 (Actor|GetActorOfClass "/Game/Blueprints/Managers/BP_WaveManager.BP_WaveManager_C"))
          (Utilities|IsValid _returnvalue_2
            (:Is%20Valid
              (Variables|Default|SetWaveManager _returnvalue_2))
            (:Is%20Not%20Valid
              (bind _returnvalue_3 (Game|SpawnActorfromClass "/Game/Blueprints/Managers/BP_WaveManager.BP_WaveManager_C" (Math|Transform|MakeTransform "616.000000,616.000000,616.000000" "0, 0, 0" "1.000000,1.000000,1.000000") "AlwaysSpawn" "OverrideRootScale" 0 0))
              (Variables|Default|SetWaveManager _returnvalue_3))))))
    (:then_2
      (Default|OnKilledEnemy (Variables|Default|GetWaveManager) self (Variables|Default|GetbKilledByPlayer)))
    (:then_3
      (Niagara|SpawnSystematLocation "/Game/Art/Particles/PS_PlaceholderExplosion.PS_PlaceholderExplosion" (Transformation|GetActorLocation) "0, 0, 0" "1.000000,1.000000,1.000000" true true "AutoRelease"))
    (:then_4
      (Widget|RemovefromParent _hpbar)
      (Widget|SetIsEnabled _hpbar false)
      (Widget|SetVisibility _hpbar "Collapsed")
      (if (Rendering|IsVisible (Variables|Default|GetPLACEHOLDER_MESH))
        ;[1 1 1] Spawn explosion
        (|CallParentFunction :!label _label)
        (Effects|SpawnEmitteratLocation "/Game/StarterContent/Particles/P_Explosion.P_Explosion" "0, 0, 0" "0, 0, 0" "5.000000,5.000000,5.000000" true "AutoRelease")
        (else
          (Variables|Default|SetbIsDead true)
          (if (Variables|Default|GetbKilledByPlayer)
            ;[1 1 1] SetDead
            (Utilities|IsValid _returnvalue
              (:Is%20Valid
                (AI|Navigation|StopMovement _returnvalue)))
            (else
              (goto _label))))))))

(fn CheckPlayerinRange
  (Utilities|IsValid (Variables|Default|GetPlayerActor)
    (:Is%20Valid
      (return (<= (Math|Float|Absolute(Float) (Math|Vector|Distance2D(Vector) (Transformation|GetWorldLocation (Variables|Default|GetCapsuleComponent)) (Transformation|GetWorldLocation (Variables|/Script/Engine.Character|GetCapsuleComponent (Variables|Default|GetPlayerActor))))) (Variables|Default|GetAttackRange))))))

(fn CheckAttackAvailable
  (bind _inrange (CallFunction|CheckPlayerinRange))
  (return (and _inrange (Variables|Default|GetbCanAttack))))

(fn CheckStartSlow
  (params (Actor :type Actor%20Object%20Reference))
  (bind _returnvalue (Actor|GetComponentbyClass Actor "/Game/Blueprints/Projectiles/HeroSkills/BP_SlowEffectorComponent.BP_SlowEffectorComponent_C"))
  (Utilities|IsValid Actor
    (:Is%20Valid
      (if (Utilities|IsValid _returnvalue)
        (if (not (Variables|Default|GetbIsSlowed))
          (Variables|Default|SetbIsSlowed true)
          (Variables|/Script/Engine.CharacterMovementComponent|SetMaxWalkSpeed (Variables|Character|GetCharacterMovement) (* (Variables|Default|GetDefaultMovementSpeed) (Variables|/Game/Blueprints/Projectiles/HeroSkills/BP_SlowEffectorComponent.BP_SlowEffectorComponent_C|GetSlowMultiplier _returnvalue))))))))

(fn CheckEndSlow
  (params (Actor :type Actor%20Object%20Reference))
  (Utilities|IsValid Actor
    (:Is%20Valid
      (if (and (Actor|ActorHasTag Actor "SlowEffector") (Variables|Default|GetbIsSlowed))
        (Variables|Default|SetbIsSlowed false)
        (Variables|/Script/Engine.CharacterMovementComponent|SetMaxWalkSpeed (Variables|Character|GetCharacterMovement) (Variables|Default|GetDefaultMovementSpeed))))))

(fn TakeDamage
  (params (Damage :type Float%20%28double-precision%29))
  (|CallParentFunction Damage)
  (Widget|SetVisibility (Variables|Default|GetHPBar) "Visible"))

(fn ApplySlow
  (params (SlowMultiplier :type Float%20%28double-precision%29) (Slow :type Boolean))
  (LocalVariables|SetSlowMultip SlowMultiplier)
  (if Slow
    (if (not (Variables|Default|GetbIsSlowed))
      (Variables|Default|SetbIsSlowed true)
      (Variables|/Script/Engine.CharacterMovementComponent|SetMaxWalkSpeed (Variables|Character|GetCharacterMovement) (* (Variables|Default|GetDefaultMovementSpeed) (LocalVariables|GetSlowMultip))))
    (elif (Variables|Default|GetbIsSlowed)
      (Variables|Default|SetbIsSlowed false)
      (Variables|/Script/Engine.CharacterMovementComponent|SetMaxWalkSpeed (Variables|Character|GetCharacterMovement) (Variables|Default|GetDefaultMovementSpeed)))))