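; BP_EntityBase is a character entity Blueprint, apparently meant as a base class, that gives actors basic health and death handling.
; BeginPlay sets current HP to the maximum, and AnyDamage subtracts incoming damage, destroying the actor once HP reaches zero or below.
; A getter returns current HP, max HP and their ratio.
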(event EventBeginPlay
  (CallFunction|InitializeEntity))

(event Game|Damage|EventAnyDamage
  (params (Damage :type Float%20%28single-precision%29) (DamageType :type Damage%20Type%20Object%20Reference) (InstigatedBy :type Controller%20Object%20Reference) (DamageCauser :type Actor%20Object%20Reference))
  (CallFunction|TakeDamage Damage))

(fn ConstructionScript)

(fn InitializeEntity
  (Variables|Default|Set_currentHP (Variables|Default|GetMaxHP)))

(fn TakeDamage
  (params (Damage :type Float%20%28double-precision%29))
  (bind _output_get (Variables|Default|Set_currentHP (- (Variables|Default|Get_currentHP) Damage)))
  (if (<= _output_get 0.0)
    (CallFunction|Die)))

(fn Die
  (Actor|DestroyActor))

(fn GetHPValues
  (return (Variables|Default|Get_currentHP) (Variables|Default|GetMaxHP) (/ (Variables|Default|Get_currentHP) (Variables|Default|GetMaxHP))))