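; Molotov projectile for the Scorcher boss, built on a damageable enemy-style parent with an HP bar.
; It tumbles every tick, ignores slow, stun and knockback, and passes every hit to the parent as 1 damage.
; BeginPlay finds or spawns the wave manager and plays a spawn sound.
; On death, effects and sound depend on whether the player killed it, then it notifies the wave manager as a non-objective kill and destroys itself.
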(event EventBeginPlay
  (Utilities|FlowControl|Sequence
    (:then_0
      (bind _returnvalue (Actor|GetActorOfClass "/Game/Blueprints/Managers/BP_WaveManager.BP_WaveManager_C"))
      (Utilities|IsValid _returnvalue
        (:Is%20Valid
          (Variables|Default|SetWaveManager _returnvalue))
        (:Is%20Not%20Valid
          (bind _returnvalue_2 (Game|SpawnActorfromClass "/Game/Blueprints/Managers/BP_WaveManager.BP_WaveManager_C" (Math|Transform|MakeTransform "666.000000,666.000000,666.000000" "0, 0, 0" "1.000000,1.000000,1.000000") "Undefined" "MultiplyWithRoot" 0 0))
          (Variables|Default|SetWaveManager _returnvalue_2))))
    (:then_1
      (|CallParentFunction)
      (Audio|PlaySound2D (Variables|Default|GetSpawnSound) 1.0 1.0 0.0 0 0))))

(event EventOnSlowApplied
  (params (SlowMultiplier :type Float%20%28double-precision%29) (isSlowed :type Boolean))
  ;[1 1 1] No slow, stun or knockback
)

(event EventOnStun
  (params (Duration :type Float%20%28double-precision%29))
  ;[1 1 1] No slow, stun or knockback
)

(event EventApplyKnockback
  (params (ForceVector :type Vector :default "0, 0, 0"))
  ;[1 1 1] No slow, stun or knockback
)

(event EventTick
  (params (DeltaSeconds :type Float%20%28single-precision%29))
  (|CallParentFunction DeltaSeconds)
  (CallFunction|RotateMesh DeltaSeconds))

(fn ConstructionScript
  (|CallParentFunction))

(fn RotateMesh
  (params (DeltaTime :type Float%20%28double-precision%29))
  (bind _returnvalue (* DeltaTime 225.0))
  (bind _placeholder_mesh (Variables|Default|GetPLACEHOLDER_MESH)
    (:then
      (Transformation|AddLocalRotation _placeholder_mesh (Math|Rotator|MakeRotator _returnvalue _returnvalue _returnvalue) false false))
    (:else)))

(fn TakeDamage
  (params (Damage :type Float%20%28double-precision%29))
  (|CallParentFunction 1.0))

(fn CheckStartSlow
  (params (Actor :type Actor%20Object%20Reference)))

(fn CheckEndSlow
  (params (Actor :type Actor%20Object%20Reference)))

(fn Die
  (bind _returnvalue (Transformation|GetActorLocation))
  (bind _hpbar (Variables|Default|GetHPBar))
  (Utilities|FlowControl|Sequence
    (:then_0
      (Widget|RemovefromParent _hpbar)
      (Widget|SetIsEnabled _hpbar false)
      (Widget|SetVisibility _hpbar "Collapsed"))
    (:then_1
      (Variables|Default|SetbIsDead true)
      (if (Variables|Default|GetbKilledByPlayer)
        (Effects|SpawnEmitteratLocation "/Game/Characters/IggyScorchBoss/FX/Particles/IggyScorch/Abilities/Primary/FX/P_IggyScorch_Molotov_HitWorld.P_IggyScorch_Molotov_HitWorld" _returnvalue)
        (Audio|PlaySound2D (Variables|Default|GetCancelSound) 1.0 1.0 0.0 0 0)
        (else
          (Effects|SpawnEmitteratLocation "/Game/Characters/IggyScorchBoss/FX/Particles/IggyScorch/Abilities/Primary/FX/P_IggyScorch_Molotov_HitPlayer.P_IggyScorch_Molotov_HitPlayer" _returnvalue "0, 0, 0" "2.000000,2.000000,2.000000" true "AutoRelease")
          (Audio|PlaySound2D (Variables|Default|GetHitSound) 1.0 1.0 0.0 0 0))))
    (:then_2
      (Default|OnKilledEnemy (Variables|Default|GetWaveManager) self (Variables|Default|GetbKilledByPlayer) false))
    (:then_3
      (Actor|DestroyActor))))