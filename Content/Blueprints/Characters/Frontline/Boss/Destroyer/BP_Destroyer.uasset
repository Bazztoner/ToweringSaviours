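; Destroyer boss character that chases the player under a behavior tree, with its own HP bar widget.
; Attacks stop its movement and raise an attack-start event, while range checks serve light and heavy attacks.
; Damage drains a stun meter outside retreats and heavy attacks.
; Depleting it or ending an attack triggers a retreat phase: timed movement changes, then a teleport to a random spawn point, facing the player.
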(event Custom|OnStunEnd
  (CallFunction|CancelStun))

(event Custom|OnPhaseEnd
  ;[0 0 0] This event starts the retreat animation and movement
  (CallFunction|CancelStun)
  (Variables|Default|SetbIsRetreating true)
  (Variables|/Script/Engine.CharacterMovementComponent|SetMaxWalkSpeed (Variables|Character|GetCharacterMovement) (Variables|Default|GetRetreatSpeed))
  (Utilities|FlowControl|Sequence
    (:then_0
      (AI|Navigation|SimpleMovetoActor (Pawn|GetController) (Variables|Default|GetCurrentSpawnPoint))
      (bind _outactors (Actor|GetAllActorsOfClass "/Game/Blueprints/Managers/SpawnPoint.SpawnPoint_C"))
      (Variables|Default|SetNextSpawnPoint (.OutItem (Utilities|Array|Random _outactors))))
    (:then_1
      (Utilities|FlowControl|Delay 6.0)
      (Transformation|Teleport (Transformation|GetActorLocation (Variables|Default|GetNextSpawnPoint)) "0, 0, 0")
      (Transformation|SetActorRotation (Math|Conversions|RotationFromXVector (Class|KismetMathLibrary|VectorNormal2D (- (Transformation|GetActorLocation (Variables|Default|GetPlayerActor)) (Transformation|GetActorLocation)) 0.0001)))
      (Variables|Default|SetbIsRetreating false)
      (Default|CallOnRetreatEnd))
    (:then_2
      (Utilities|FlowControl|Delay 1.0)
      (Variables|/Script/Engine.CharacterMovementComponent|SetMaxWalkSpeed (Variables|Character|GetCharacterMovement) (Variables|Default|GetDefaultMovementSpeed))
      (AI|Navigation|SimpleMovetoActor (Pawn|GetController) (Variables|Default|GetPlayerActor)))))

(event Custom|OnAttackEnd
  (Variables|Default|SetbIsAttacking false)
  (CallFunction|OnPhaseEnd))

(event EventOnStun
  (params (Duration :type Float%20%28double-precision%29))
  (if (not (Variables|Default|GetbIsRetreating))
    (Variables|Default|SetbIsStunned true)
    (Variables|/Script/Engine.CharacterMovementComponent|SetMaxWalkSpeed (Variables|Character|GetCharacterMovement) 0.0)
    (Utilities|FlowControl|Delay 5.0)
    (CallFunction|OnStunEnd)))

(event EventApplyKnockback
  (params (ForceVector :type Vector :default "0, 0, 0"))
  ;[0 0 0] Knockback is stun
  (CallFunction|OnStun 1.0))

(event EventBeginPlay
  (bind _output_get (Variables|Default|SetPlayerActor (Variables|/Game/Blueprints/Player/BP_PlayerController.BP_PlayerController_C|GetPlayerCharacter (CallFunction|GetFrontlinePlayerController))))
  (CallFunction|InitializeHPBar)
  (bind _output_get_2 (Variables|Default|SetAIController (.AsAIC%20Destroyer%20Boss (Utilities|Casting|CastToAIC_DestroyerBoss (Pawn|GetController)))))
  (AI|Navigation|SimpleMovetoActor _output_get_2 _output_get)
  (AI|RunBehaviorTree (Variables|Default|GetAIController) "/Game/Blueprints/Characters/Frontline/Boss/Destroyer/BT_DestroyerBoss.BT_DestroyerBoss"))

(event EventTick
  (params (DeltaSeconds :type Float%20%28single-precision%29))
  ;[1 1 1] HARDCODEALA PA
)

(fn ConstructionScript
  (|CallParentFunction))

(fn CancelStun
  (Variables|Default|SetbIsStunned false)
  (Variables|/Script/Engine.CharacterMovementComponent|SetMaxWalkSpeed (Variables|Character|GetCharacterMovement) (Variables|Default|GetDefaultMovementSpeed)))

(fn GetAttackRange
  (params (HeavyAttack :type Boolean))
  (bind _returnvalue (Transformation|GetActorLocation))
  (bind _playeractor (Variables|Default|GetPlayerActor))
  (bind _returnvalue_2 (Transformation|GetActorLocation _playeractor))
  (bind _returnvalue_3 (Math|Vector|Distance2D(Vector) _returnvalue _returnvalue_2))
  (bind _returnvalue_4 (Math|Float|Absolute(Float) _returnvalue_3))
  (if HeavyAttack
    (return _returnvalue_4 (Variables|Default|GetHeavyAttackRange))
    (else
      (return _returnvalue_4 (Variables|Default|GetAttackRange)))))

(fn SpawnLightAttack)

(fn SpawnHeavyAttack)

(fn TakeDamage
  (params (Damage :type Float%20%28double-precision%29))
  (|CallParentFunction Damage)
  (if (and (not (Variables|Default|GetbIsRetreating)) (not (Variables|Default|GetbIsAttacking)))
    (bind _output_get (Variables|Default|Set_currentStunDamage (- (Variables|Default|Get_currentStunDamage) Damage)))
    (Default|ReportStaminaChange (Variables|Default|GetBossHPWidget) _output_get (Variables|Default|GetStunDamage))
    (if (<= _output_get 0.0)
      (CallFunction|OnStun 5.0)
      (CallFunction|OnPhaseEnd))))

(fn ExecuteAttack
  (params (bIsHeavyAttack :type Boolean))
  (bind _output_get (Variables|Default|SetbIsHeavyAttack bIsHeavyAttack))
  (Variables|Default|SetbIsAttacking _output_get)
  (Default|CallOnAttackStart _output_get)
  (Components|Movement|StopMovementImmediately (Variables|Character|GetCharacterMovement)))

(fn InitializeHPBar
  (bind _returnvalue (UserInterface|CreateWidget "/Game/Blueprints/Widgets/Frontline/HUD_BossHPBar.HUD_BossHPBar_C" 0 self (Variables|Default|GetBossName)))
  (bind _output_get (Variables|Default|SetBossHPWidget _returnvalue))
  (UserInterface|Viewport|AddtoViewport _output_get 1)
  (|CallParentFunction))