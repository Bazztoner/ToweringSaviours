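; Iggy Scorch boss character that fights with molotov and fire breath attacks, driven by BT_IggyScorchBoss.
; Attack functions set readiness and busy flags, with per-attack cooldowns plus a random shared cooldown gating CheckCanAttack.
; Separate events spawn projectiles; a fire breath player hit jumps the montage to its End section.
; Damage during breath stuns the boss and cancels the attack, while knockback applies a shorter stun.
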(event Custom|SpawnBoss)

(event Custom|OnBreathAttackEnd
  (Variables|Default|SetbIsAttacking false)
  (Variables|Default|SetbIsBreathAttack false)
  (Animation|StopAnimMontage "/Game/Characters/IggyScorchBoss/Mesh/AM_IggyScorchBreathAttack.AM_IggyScorchBreathAttack")
  (CallFunction|AttackCooldownHandler)
  (Utilities|FlowControl|Delay (Variables|Default|GetBreathAttackCooldown))
  (Variables|Default|SetbBreathReady true))

(event Custom|AttackCooldownHandler
  (Utilities|FlowControl|Delay (Math|Random|RandomFloatinRange (Variables|Default|GetAttackCooldown) (Variables|Default|GetBreathAttackCooldown)))
  (Variables|Default|SetbCanAttack true))

(event Custom|OnMolotovAttackEnd
  (Variables|Default|SetbIsAttacking false)
  (CallFunction|AttackCooldownHandler)
  (Utilities|FlowControl|Delay (Variables|Default|GetAttackCooldown))
  (Variables|Default|SetbMolotovReady true))

(event Custom|SpawnBreathProjectile
  (bind _self self)
  (bind _returnvalue (Game|SpawnActorfromClass "/Game/Blueprints/Characters/Frontline/Boss/BP_FireBreath.BP_FireBreath_C" (Math|Transform|MakeTransform (Transformation|GetWorldLocation (Variables|Default|GetAttackSpawnPos)) (Math|Conversions|RotationFromXVector (Transformation|GetActorForwardVector)) "1.000000,1.000000,1.000000") "Undefined" "MultiplyWithRoot" _self _self))
  (EventDispatchers|AssignOnPlayerHit _returnvalue (delegate Custom|OnBreathHit)))

(event Custom|OnBreathHit
  (CallFunction|BreathAttackConnected)
  (EventDispatchers|UnbindEventfromOnPlayerHit (stale Custom|SpawnBreathProjectile _returnvalue) (delegate Custom|OnBreathHit)))

(event EventBeginPlay
  (Variables|Default|SetPlayerActor (Variables|/Game/Blueprints/Player/BP_PlayerController.BP_PlayerController_C|GetPlayerCharacter (CallFunction|GetFrontlinePlayerController)))
  ;[1 0.5885 0] Delay for spawn animation to complete
  (CallFunction|InitializeHPBar)
  (AI|RunBehaviorTree (AI|GetAIController self) "/Game/Blueprints/Characters/Frontline/Boss/BT_IggyScorchBoss.BT_IggyScorchBoss")
  (Utilities|FlowControl|Delay 2.0)
  (Variables|Default|SetbMolotovReady true)
  (Variables|Default|SetbBreathReady true))

(event EventTick
  (params (DeltaSeconds :type Float%20%28single-precision%29)))

(event EventApplyKnockback
  (params (ForceVector :type Vector :default "0, 0, 0"))
  (CallFunction|OnStun 0.5))

(event EventOnStun
  (params (Duration :type Float%20%28double-precision%29))
  (Variables|Default|SetbIsStunned true)
  (Utilities|FlowControl|Sequence
    (:then_0
      (if (Variables|Default|GetbIsBreathAttack)
        (CallFunction|OnBreathAttackEnd)))
    (:then_1
      (Default|CallOnBossStun))
    (:then_2
      (Utilities|FlowControl|Delay Duration)
      ;[1 1 1] Set a max stun duration later
      (Variables|Default|SetbIsStunned false))))

(event EventOnSlowApplied
  (params (SlowMultiplier :type Float%20%28double-precision%29) (isSlowed :type Boolean))
  ;[1 1 1] Nothing
)

(fn ConstructionScript
  (|CallParentFunction))

(fn InitializeHPBar
  (|CallParentFunction))

(fn GetHPRange
  (bind _returnvalue (Math|Float|MakeLiteralFloat 1.0))
  (bind _currenthpbar (Variables|Default|GetCurrentHPBar))
  (bind _hpbars (Variables|Default|GetHPBars))
  (bind _returnvalue_2 (/ _returnvalue _hpbars))
  (bind _returnvalue_3 (* _currenthpbar _returnvalue_2))
  (return (- _returnvalue_3 _returnvalue_2) _returnvalue_3))

(fn SpawnMolotovProjectile
  (Game|SpawnActorfromClass "/Game/Blueprints/Characters/Frontline/Boss/BP_MolotovProjectile.BP_MolotovProjectile_C" (Math|Transform|MakeTransform (Transformation|GetWorldLocation (Variables|Default|GetAttackSpawnPos)) (Math|Conversions|RotationFromXVector (Transformation|GetActorForwardVector)) "1.000000,1.000000,1.000000") "Undefined" "MultiplyWithRoot" 0 0 0))

(fn Attack)

(fn TakeDamage
  (params (Damage :type Float%20%28double-precision%29))
  (|CallParentFunction Damage)
  (if (Variables|Default|GetbIsBreathAttack)
    (CallFunction|OnStun 2.0)))

(fn CheckCanAttack
  (return (Math|Boolean|ANDBoolean (not (Variables|Default|GetbIsDead)) (not (Variables|Default|GetbIsStunned)) (Variables|Default|GetbCanAttack))))

(fn MolotovAttack
  (Variables|Default|SetbIsAttacking true)
  (Variables|Default|SetbMolotovReady false)
  (Variables|Default|SetbCanAttack false))

(fn BreathAttack
  (if (not (Variables|Default|GetbIsAttacking))
    (Variables|Default|SetbIsAttacking true)
    (Variables|Default|SetbIsBreathAttack true)
    (Variables|Default|SetbCanAttack false)
    (Animation|PlayAnimMontage "/Game/Characters/IggyScorchBoss/Mesh/AM_IggyScorchBreathAttack.AM_IggyScorchBreathAttack" 1.0 "None")
    (Variables|Default|SetbBreathReady false)))

(fn BreathAttackConnected
  (Animation|PlayAnimMontage "/Game/Characters/IggyScorchBoss/Mesh/AM_IggyScorchBreathAttack.AM_IggyScorchBreathAttack" 1.0 "End"))