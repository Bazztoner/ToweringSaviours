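; Game instance for a wave-based hero game, holding run state, hero choice and persistent stats across levels.
; Save merges the current wave and kill counts into overall and per-hero bests and totals, then writes them to one BP_SaveGame slot.
; Hero selection returns the picked class or a random one of three.
; It also drives the loading screen, platform detection, level-wall lookup and music that persists through level transitions.
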(event Custom|Save
  (Utilities|IsValid (Variables|Default|GetSaveGame)
    (:Is%20Valid
      _)
    (:Is%20Not%20Valid
      (bind _returnvalue (SaveGame|CreateSaveGameObject "/Game/Blueprints/Managers/SaveGame/BP_SaveGame.BP_SaveGame_C"))
      (Variables|Default|SetSaveGame _returnvalue)))
  (bind (_maxenemieskilled _maxwavereached _enemieskilledtotal) (CallFunction|GetPlayerStats))
  (CallFunction|SavePlayerStats _maxenemieskilled _maxwavereached _enemieskilledtotal)
  (bind (_heromaxenemies _heromaxwave _herototalenemies) (CallFunction|GetHeroStats))
  (CallFunction|SaveHeroStats _heromaxenemies _heromaxwave _herototalenemies)
  (bind _herocharacterpicked (CallFunction|GetPlayerCharacter))
  (Variables|/Game/Blueprints/Managers/SaveGame/BP_SaveGame.BP_SaveGame_C|SetLastHeroUsed (Variables|Default|GetSaveGame) _herocharacterpicked)
  (SaveGame|SaveGametoSlot (Variables|Default|GetSaveGame) "savegame"))

(event Custom|ResetStats
  (Default|ResetStats (Variables|Default|GetSaveGame))
  (SaveGame|SaveGametoSlot (Variables|Default|GetSaveGame) "savegame"))

(event Custom|Load
  (bind _returnvalue (SaveGame|DoesSaveGameExist "savegame"))
  (if _returnvalue
    (bind _returnvalue_2 (SaveGame|LoadGamefromSlot "savegame"))
    (bind _asbp_save_game (Utilities|Casting|CastToBP_SaveGame _returnvalue_2))
    (Variables|Default|SetSaveGame _asbp_save_game)
    (else
      (bind _returnvalue_3 (SaveGame|CreateSaveGameObject "/Game/Blueprints/Managers/SaveGame/BP_SaveGame.BP_SaveGame_C"))
      (Variables|Default|SetSaveGame _returnvalue_3))))

(event Custom|OnLoadStart
  (bind _returnvalue (UserInterface|CreateWidget "/Game/Blueprints/Widgets/WBP_LoadingScreen.WBP_LoadingScreen_C"))
  (bind _output_get (Variables|Default|SetLoadingScreen _returnvalue))
  (UserInterface|Viewport|AddtoViewport _output_get 2))

(event Custom|OnLoadEnd
  (Widget|RemovefromParent (Variables|Default|GetLoadingScreen)))

(event Custom|DelayedLoad
  (params (Delay :type Float%20%28double-precision%29))
  (CallFunction|OnLoadStart)
  (Utilities|FlowControl|Delay Delay)
  (CallFunction|OnLoadEnd))

(fn GetPlayerCharacter
  (if (Variables|Default|GetRandomCharacter)
    (return (Utilities|Select :Index (Math|Random|RandomIntegerinRange 0 2) :Option%200 "/Game/Blueprints/Characters/Frontline/Hero/BP_HeroAssassin.BP_HeroAssassin_C" :Option%201 "/Game/Blueprints/Characters/Frontline/Hero/BP_HeroMage.BP_HeroMage_C" :Option%202 "/Game/Blueprints/Characters/Frontline/Hero/BP_HeroDemolisher.BP_HeroDemolisher_C"))
    (else
      (return (Variables|Default|GetHeroCharacterPicked)))))

(fn ChangeWave
  (params (CurrentWave :type Integer) (EnemiesInWave :type Integer))
  (Variables|Default|SetCurrentWave CurrentWave)
  (Variables|Default|SetEnemiesInWave EnemiesInWave)
  (Variables|Default|SetEnemiesKilledWave 0))

(fn RestartGame
  (bind _output_get (Variables|Default|SetEnemiesKilledTotal 0))
  (bind _output_get_2 (Variables|Default|SetEnemiesKilledWave _output_get))
  (bind _output_get_3 (Variables|Default|SetEnemiesInWave _output_get_2))
  (Variables|Default|SetCurrentWave _output_get_3))

(fn PickCharacter
  (params (HeroCharacterPicked :type BP%20Hero%20Base%20Class%20Reference))
  (Variables|Default|SetRandomCharacter false)
  (Variables|Default|SetHeroCharacterPicked HeroCharacterPicked))

(fn GetCurrentPlatform
  (Utilities|FlowControl|Sequence
    (:then_1
      (switch string (Game|GetPlatformName)
        (:Default
          (LocalVariables|SetPlatform "NewEnumerator0" :!label _label))
        (:Windows
          (goto _label))
        (:Mac
          (goto _label))
        (:Linux
          (goto _label))
        (:Android
          (LocalVariables|SetPlatform "NewEnumerator1" :!label _label_2))
        (:iOS
          (goto _label_2))))
    (:then_2
      (return (LocalVariables|GetPlatform)))))

(fn GetLevelWalls
  (bind _outactors (Actor|GetAllActorswithTag "LevelWall"))
  (bind _output_get (Variables|Default|SetLevelWalls _outactors))
  (return _output_get))

(fn GetPlayerStats
  (bind _savegame (Variables|Default|GetSaveGame))
  (bind _enemieskilledtotal (Variables|Default|GetEnemiesKilledTotal))
  (bind _currentwave (Variables|Default|GetCurrentWave))
  (bind _maxenemieskilled (Variables|/Game/Blueprints/Managers/SaveGame/BP_SaveGame.BP_SaveGame_C|GetMaxEnemiesKilled _savegame))
  (bind _maxwavereached (Variables|/Game/Blueprints/Managers/SaveGame/BP_SaveGame.BP_SaveGame_C|GetMaxWaveReached _savegame))
  (Utilities|FlowControl|Sequence
    (:then_0
      (if (> _enemieskilledtotal _maxenemieskilled)
        (LocalVariables|SetMaxKilled _enemieskilledtotal)
        (else
          (LocalVariables|SetMaxKilled _maxenemieskilled))))
    (:then_1
      (if (> _currentwave _maxwavereached)
        (LocalVariables|SetMaxWave _currentwave)
        (else
          (LocalVariables|SetMaxWave _maxwavereached))))
    (:then_2
      (LocalVariables|SetKilledTotal (+ (Variables|/Game/Blueprints/Managers/SaveGame/BP_SaveGame.BP_SaveGame_C|GetEnemiesKilledTotal _savegame) (Variables|Default|GetEnemiesKilledTotal))))
    (:then_3
      (return (LocalVariables|GetMaxKilled) (LocalVariables|GetMaxWave) (LocalVariables|GetKilledTotal)))))

(fn GetHeroStats
  (bind _herocharacterpicked (Variables|Default|GetHeroCharacterPicked))
  (bind _savegame (Variables|Default|GetSaveGame))
  (bind _enemieskilledtotal (Variables|Default|GetEnemiesKilledTotal))
  (bind _enemieskilledtotal_2 (Variables|Default|GetEnemiesKilledTotal))
  (bind _currentwave (Variables|Default|GetCurrentWave))
  (bind _herocharacterpicked_2 (Variables|Default|GetHeroCharacterPicked))
  (bind _herocharacterpicked_3 (Variables|Default|GetHeroCharacterPicked))
  (bind _herowavereached (Variables|/Game/Blueprints/Managers/SaveGame/BP_SaveGame.BP_SaveGame_C|GetHeroWaveReached _savegame))
  (bind _heroenemiesmaxkilled (Variables|/Game/Blueprints/Managers/SaveGame/BP_SaveGame.BP_SaveGame_C|GetHeroEnemiesMaxKilled _savegame))
  (bind _heroenemiestotalkilled (Variables|/Game/Blueprints/Managers/SaveGame/BP_SaveGame.BP_SaveGame_C|GetHeroEnemiesTotalKilled _savegame))
  (bind (_value _returnvalue) (Utilities|Map|Find _herowavereached _herocharacterpicked))
  (bind (_value_2 _returnvalue_2) (Utilities|Map|Find _heroenemiesmaxkilled _herocharacterpicked_3))
  (bind (_value_3 _returnvalue_3) (Utilities|Map|Find _heroenemiestotalkilled _herocharacterpicked_2))
  (Utilities|FlowControl|Sequence
    (:then_0
      (if _returnvalue
        (if (> _currentwave _value)
          (LocalVariables|SetCurrentHeroMaxWave _currentwave :!label _label)
          (else
            (LocalVariables|SetCurrentHeroMaxWave _value)))
        (else
          (goto _label))))
    (:then_1
      (if _returnvalue_2
        (if (> _enemieskilledtotal _value_2)
          (LocalVariables|SetCurrentHeroMaxEnemies _enemieskilledtotal :!label _label_2)
          (else
            (LocalVariables|SetCurrentHeroMaxEnemies _value_2)))
        (else
          (goto _label_2))))
    (:then_2
      (if _returnvalue_3
        (LocalVariables|SetCurrentHeroTotalEnemies (+ _enemieskilledtotal_2 _value_3))
        (else
          (LocalVariables|SetCurrentHeroTotalEnemies (Class|KismetMathLibrary|ToInt64(Integer) _enemieskilledtotal_2)))))
    (:then_3
      (return (LocalVariables|GetCurrentHeroMaxEnemies) (LocalVariables|GetCurrentHeroMaxWave) (LocalVariables|GetCurrentHeroTotalEnemies)))))

(fn SavePlayerStats
  (params (MaxEnemiesKilled :type Integer) (MaxWaveReached :type Integer) (EnemiesKilledTotal :type Integer64))
  (bind _savegame (Variables|Default|GetSaveGame))
  (Variables|/Game/Blueprints/Managers/SaveGame/BP_SaveGame.BP_SaveGame_C|SetMaxEnemiesKilled _savegame MaxEnemiesKilled)
  (Variables|/Game/Blueprints/Managers/SaveGame/BP_SaveGame.BP_SaveGame_C|SetMaxWaveReached _savegame MaxWaveReached)
  (Variables|/Game/Blueprints/Managers/SaveGame/BP_SaveGame.BP_SaveGame_C|SetEnemiesKilledTotal _savegame EnemiesKilledTotal))

(fn SaveHeroStats
  (params (MaxHeroKills :type Integer) (MaxHeroWave :type Integer) (TotalHeroKills :type Integer64))
  (bind _savegame (Variables|Default|GetSaveGame))
  (bind _herocharacterpicked (Variables|Default|GetHeroCharacterPicked))
  (Utilities|Map|Add (Variables|/Game/Blueprints/Managers/SaveGame/BP_SaveGame.BP_SaveGame_C|GetHeroEnemiesMaxKilled _savegame) _herocharacterpicked MaxHeroKills)
  (Utilities|Map|Add (Variables|/Game/Blueprints/Managers/SaveGame/BP_SaveGame.BP_SaveGame_C|GetHeroWaveReached _savegame) _herocharacterpicked MaxHeroWave)
  (Utilities|Map|Add (Variables|/Game/Blueprints/Managers/SaveGame/BP_SaveGame.BP_SaveGame_C|GetHeroEnemiesTotalKilled _savegame) _herocharacterpicked TotalHeroKills))

(fn SaveLastHeroUsed
  (bind _herocharacterpicked (CallFunction|GetPlayerCharacter))
  (bind _savegame (Variables|Default|GetSaveGame)
    (:then
      (Variables|/Game/Blueprints/Managers/SaveGame/BP_SaveGame.BP_SaveGame_C|SetLastHeroUsed _savegame _herocharacterpicked)
      (SaveGame|SaveGametoSlot _savegame "savegame"))
    (:else)))

(fn ChangeMusic
  (params (NewMusic :type Sound%20Cue%20Object%20Reference))
  (if (not (== NewMusic (Variables|Default|GetCurrentMusic)))
    (bind _musiccontroller (Variables|Default|GetMusicController)
      (:then
        (Audio|Components|Audio|Stop _musiccontroller)
        (Audio|Components|Audio|SetSound _musiccontroller NewMusic)
        (Audio|Components|Audio|Play _musiccontroller 0.0))
      (:else
        (bind _returnvalue (Audio|CreateSound2D NewMusic 1.0 1.0 0.0 0 true false))
        (bind _output_get (Variables|Default|SetMusicController _returnvalue))
        (Audio|Components|Audio|Play _output_get 0.0)))
    (Variables|Default|SetCurrentMusic NewMusic)))