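; Wave manager that runs an endless sequence of normal and boss enemy waves.
; Each wave is a BP_WaveClass actor with weighted enemy tables; finishing one appends another, with every sixth a boss wave.
; A looping timer spawns objective enemies near random spawn points up to an active cap; boss waves add timed fodder.
; It also tracks kills, awards player mana, provides nearest-enemy lookup, and switches music between boss and normal waves.
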(event Custom|FinishWave
  (Utilities|Time|ClearandInvalidateTimerbyHandle (Variables|Default|GetFodderSpawnTimer))
  (Utilities|FlowControl|Delay (Variables|Default|GetWaveChangeDelay))
  (CallFunction|ChangetoNextWave)
  (CallFunction|AddNextWave))

(event Custom|EnemySpawnHandler
  (CallFunction|SpawnEnemyObjective))

(event Custom|OnBossWave
  (bind _returnvalue (Utilities|Time|SetTimerbyEvent (delegate Custom|SpawnFodderEnemies) (Variables|Default|GetFodderSpawnCooldown) true))
  (Variables|Default|SetFodderSpawnTimer _returnvalue))

(event Custom|SpawnFodderEnemies
  (CallFunction|SpawnEnemyFodder))

(event EventBeginPlay
  (Utilities|FlowControl|DelayUntilNextTick)
  (Variables|/Game/Blueprints/Characters/Frontline/Hero/BP_HeroBase.BP_HeroBase_C|SetWaveManager (Variables|/Game/Blueprints/Player/BP_PlayerController.BP_PlayerController_C|GetPlayerCharacter (CallFunction|GetFrontlinePlayerController)) self)
  (Utilities|FlowControl|Sequence
    (:then_0
      (bind _outactors (Actor|GetAllActorsOfClass "/Game/Blueprints/Managers/SpawnPoint.SpawnPoint_C"))
      (Variables|Default|SetSpawnPoints _outactors))
    (:then_1
      (CallFunction|CreateStartingWaves)
      (Utilities|FlowControl|DelayUntilNextTick)
      (CallFunction|ChangetoNextWave))
    (:then_2
      (Utilities|Time|SetTimerbyEvent (delegate Custom|EnemySpawnHandler) (Variables|Default|GetSpawnCooldown) true))))

(fn ConstructionScript)

(fn OnKilledEnemy
  (params (EnemyKilled :type BP%20Enemy%20Base%20Object%20Reference) (KilledByPlayer :type Boolean) (WaveObjective :type Boolean))
  (bind _gameinstancefrontline (CallFunction|GetFrontlineGameInstance))
  (Utilities|FlowControl|Sequence
    (:then_0
      (LocalVariables|SetEnemy EnemyKilled)
      (LocalVariables|SetByPlayer KilledByPlayer)
      (LocalVariables|SetIsObjective WaveObjective))
    (:then_1
      (Utilities|IsValid (LocalVariables|GetEnemy)
        (:Is%20Valid
          (Utilities|Array|RemoveItem (Variables|Default|GetActiveEnemies) (LocalVariables|GetEnemy)))))
    (:then_2
      (if (LocalVariables|GetByPlayer)
        (CallFunction|OnPlayerKilledEnemy (LocalVariables|GetEnemy))))
    (:then_3
      (Math|Integer|IncrementInt (Variables|/Game/Blueprints/Managers/GI_Frontline.GI_Frontline_C|GetEnemiesKilledTotal _gameinstancefrontline)
        (:%20%20
          (if (LocalVariables|GetIsObjective)
            (Math|Integer|IncrementInt (Variables|/Game/Blueprints/Managers/GI_Frontline.GI_Frontline_C|GetEnemiesKilledWave _gameinstancefrontline))))))
    (:then_4
      (if (LocalVariables|GetIsObjective)
        (bind _wave_clear (Default|OnEnemyDeath (Utilities|Array|Get(acopy) (Variables|Default|GetAllWaves) (Variables|Default|GetCurrentWave))))
        (if _wave_clear
          (CallFunction|FinishWave))))))

(fn OnPlayerKilledEnemy
  (params (EnemyKilled :type BP%20Enemy%20Base%20Object%20Reference))
  (Default|OnEnemyKilled (CallFunction|GetFrontlinePlayerController) (Variables|/Game/Blueprints/Characters/Frontline/Enemy/BP_EnemyBase.BP_EnemyBase_C|GetManaGrantedOnKill EnemyKilled))
  (Game|SpawnActorfromClass "/Game/Blueprints/Misc/BP_3DText.BP_3DText_C" (Math|Transform|MakeTransform (+ (Transformation|GetActorLocation EnemyKilled) "0,0,200.000000") "0, 0, 0" "1.000000,1.000000,1.000000") "AlwaysSpawn" "OverrideRootScale" 0 (Utilities|Text|ToText(String) (Utilities|String|Append "+" (Utilities|String|ToString(Integer) (Variables|/Game/Blueprints/Characters/Frontline/Enemy/BP_EnemyBase.BP_EnemyBase_C|GetManaGrantedOnKill EnemyKilled)))) "(R=0.000000,G=0.925979,B=1.000000,A=1.000000)" 0))

(fn SpawnEnemyObjective
  (bind _output_get (LocalVariables|SetWaveObject (Utilities|Array|Get(acopy) (Variables|Default|GetAllWaves) (Variables|Default|GetCurrentWave))))
  (bind _space_available (Default|GetEnemyObjectiveAmount _output_get))
  (if (and _space_available (< (Utilities|Array|Length (Variables|Default|GetActiveEnemies)) (Variables|Default|GetMaxActiveEnemies)))
    (bind _enemyclass (Default|GetEnemyObjective (LocalVariables|GetWaveObject)))
    (bind (_randomlocation _return_value_rotation) (CallFunction|GetRandomSpawnPoint))
    (bind _returnvalue (Game|SpawnActorfromClass _enemyclass (Math|Transform|MakeTransform _randomlocation _return_value_rotation "1.000000,1.000000,1.000000") "AlwaysSpawn" "SelectDefaultAtRuntime" 0 self true 0))
    (Utilities|Array|Add (Variables|Default|GetActiveEnemies) _returnvalue)
    (Default|AddEnemyObjective (LocalVariables|GetWaveObject) _returnvalue)
    (Utilities|Array|SetArrayElem (Variables|Default|GetAllWaves) (Variables|Default|GetCurrentWave) (LocalVariables|GetWaveObject) true)
    (Math|Integer|IncrementInt (Variables|Default|GetSpawnedEnemies))))

(fn SpawnEnemyFodder
  (bind _output_get (LocalVariables|SetWaveObject (Utilities|Array|Get(acopy) (Variables|Default|GetAllWaves) (Variables|Default|GetCurrentWave))))
  (for _index (range 0 (.TotalEnemies (Utilities|Struct|BreakSTRUCT_WaveData (Variables|/Game/Blueprints/Managers/WaveSystem/BP_WaveClass.BP_WaveClass_C|GetFodderData _output_get))))
    (bind _enemyclass (Default|GetFodder (LocalVariables|GetWaveObject)))
    (bind (_randomlocation _return_value_rotation _return_value_scale) (CallFunction|GetRandomSpawnPoint))
    (bind _returnvalue (Game|SpawnActorfromClass _enemyclass (Math|Transform|MakeTransform _randomlocation _return_value_rotation _return_value_scale) "AlwaysSpawn" "SelectDefaultAtRuntime" 0 self false 0))
    (CallFunction|RegisterFodderEnemy _returnvalue)
    (Utilities|Array|SetArrayElem (Variables|Default|GetAllWaves) (Variables|Default|GetCurrentWave) (LocalVariables|GetWaveObject) true)))

(fn GetRandomSpawnPoint
  (bind _spawnpoints (Variables|Default|GetSpawnPoints))
  (bind _outitem (Utilities|Array|Random _spawnpoints))
  (bind _returnvalue (Transformation|GetActorTransform _outitem))
  (bind _randomlocation (Class|NavigationSystemV1|GetRandomLocationinNavigableRadius (.location _returnvalue) 2.5e+02 0 0))
  (return _randomlocation (.rotation _returnvalue) (.scale _returnvalue)))

(fn FindClosestEnemy
  (bind _frontline_player_controller (CallFunction|GetFrontlinePlayerController))
  (bind _activeenemies (Variables|Default|GetActiveEnemies))
  (bind _playercharacter (Variables|/Game/Blueprints/Player/BP_PlayerController.BP_PlayerController_C|GetPlayerCharacter _frontline_player_controller))
  (bind _returnvalue (Transformation|GetActorLocation _playercharacter))
  (bind (_distance _returnvalue_2) (Actor|FindNearestActor _returnvalue _activeenemies))
  (Utilities|IsValid _frontline_player_controller
    (:Is%20Valid
      (bind _asbp_enemy_base (Utilities|Casting|CastToBP_EnemyBase _returnvalue_2))
      (if (>= (Variables|/Game/Blueprints/Characters/Frontline/Hero/BP_HeroBase.BP_HeroBase_C|GetAttackRange _playercharacter) _distance)
        (return _asbp_enemy_base)))))

(fn CreateNewWave
  (params (WaveNumber :type Integer) (EnemyAmount :type Integer))
  (bind _returnvalue (Game|SpawnActorfromClass "/Game/Blueprints/Managers/WaveSystem/BP_WaveClass.BP_WaveClass_C" (Math|Transform|MakeTransform "666.000000,666.000000,666.000000" "0, 0, 0" "1.000000,1.000000,1.000000") "AlwaysSpawn" "OverrideRootScale" 0 WaveNumber false 0))
  (Variables|/Game/Blueprints/Managers/WaveSystem/BP_WaveClass.BP_WaveClass_C|SetEnemyObjectiveData _returnvalue (Utilities|Struct|MakeSTRUCT_WaveData (Math|Integer|Clamp(Integer) EnemyAmount 1 100) (Utilities|Map|MakeMap "/Game/Blueprints/Characters/Frontline/Enemy/BP_EnemyWeak.BP_EnemyWeak_C" 50 "/Game/Blueprints/Characters/Frontline/Enemy/BP_EnemyMid.BP_EnemyMid_C" 35 "/Game/Blueprints/Characters/Frontline/Enemy/BP_EnemyStrong.BP_EnemyStrong_C" 15)))
  (Utilities|Array|AddUnique (Variables|Default|GetAllWaves) _returnvalue))

(fn CreateNewBossWave
  (params (Wave%20Number :type Integer) (BossAmount :type Integer) (BossClass :type BP%20Boss%20Base%20Class%20Reference))
  (bind _returnvalue (Game|SpawnActorfromClass "/Game/Blueprints/Managers/WaveSystem/BP_WaveClass.BP_WaveClass_C" (Math|Transform|MakeTransform "666.000000,666.000000,666.000000" "0, 0, 0" "1.000000,1.000000,1.000000") "AlwaysSpawn" "OverrideRootScale" 0 Wave%20Number true 0))
  (Variables|/Game/Blueprints/Managers/WaveSystem/BP_WaveClass.BP_WaveClass_C|SetEnemyObjectiveData _returnvalue (Utilities|Struct|MakeSTRUCT_WaveData BossAmount (Utilities|Map|MakeMap BossClass 100)))
  (Utilities|Array|AddUnique (Variables|Default|GetAllWaves) _returnvalue)
  (Variables|/Game/Blueprints/Managers/WaveSystem/BP_WaveClass.BP_WaveClass_C|SetFodderData _returnvalue (Utilities|Struct|MakeSTRUCT_WaveData (Math|Random|RandomIntegerinRange 3 7) (Utilities|Map|MakeMap "/Game/Blueprints/Characters/Frontline/Enemy/BP_EnemyWeak.BP_EnemyWeak_C" 63 "/Game/Blueprints/Characters/Frontline/Enemy/BP_EnemyMid.BP_EnemyMid_C" 35 "/Game/Blueprints/Characters/Frontline/Enemy/BP_EnemyStrong.BP_EnemyStrong_C" 2))))

(fn AddNextWave
  (bind _allwaves (Variables|Default|GetAllWaves))
  (bind _returnvalue (Utilities|Array|LastIndex _allwaves))
  (bind _output (Utilities|Array|Get(acopy) _allwaves _returnvalue))
  (bind _output_get (LocalVariables|SetNewWaveNumber (Utilities|Array|Length _allwaves)))
  (if (== (Math|Integer|%(Integer) _output_get 6) 0)
    (CallFunction|CreateNewBossWave (LocalVariables|GetNewWaveNumber) 1)
    (elif (Variables|/Game/Blueprints/Managers/WaveSystem/BP_WaveClass.BP_WaveClass_C|GetBossWave _output)
      (CallFunction|CreateNewWave (LocalVariables|GetNewWaveNumber) (Math|Random|RandomIntegerinRange 15 25))
      (else
        (bind _enemies_amount (Default|GetEnemyObjectiveAmount _output))
        (CallFunction|CreateNewWave (LocalVariables|GetNewWaveNumber) (+ _enemies_amount (Math|Random|RandomIntegerinRange -1 7)))))))

(fn CreateStartingWaves
  (CallFunction|CreateNewBossWave 1 1 "/Game/Blueprints/Characters/Frontline/Boss/BP_IggyScorchBoss.BP_IggyScorchBoss_C")
  (CallFunction|CreateNewWave 2 14)
  (CallFunction|CreateNewWave 3 18)
  (CallFunction|CreateNewWave 4 22)
  (CallFunction|CreateNewWave 5 25)
  (CallFunction|CreateNewBossWave 6 1 "/Game/Blueprints/Characters/Frontline/Boss/BP_IggyScorchBoss.BP_IggyScorchBoss_C"))

(fn ChangetoNextWave
  (Utilities|FlowControl|Sequence
    (:then_0
      (if (> (Variables|Default|GetCurrentWave) 0)
        (LocalVariables|SetCurrentWaveType (Variables|/Game/Blueprints/Managers/WaveSystem/BP_WaveClass.BP_WaveClass_C|GetBossWave (Utilities|Array|Get(acopy) (Variables|Default|GetAllWaves) (Variables|Default|GetCurrentWave))))))
    (:then_1
      (bind _result (Math|Integer|IncrementInt (Variables|Default|GetCurrentWave))
        (:%20%20
          (bind _enemies_amount (Default|GetEnemyObjectiveAmount (Utilities|Array|Get(acopy) (Variables|Default|GetAllWaves) _result)))
          (LocalVariables|SetNextWaveType (Variables|/Game/Blueprints/Managers/WaveSystem/BP_WaveClass.BP_WaveClass_C|GetBossWave (Utilities|Array|Get(acopy) (Variables|Default|GetAllWaves) _result)))
          (Default|ChangeWave (CallFunction|GetFrontlineGameInstance) (Variables|/Game/Blueprints/Managers/WaveSystem/BP_WaveClass.BP_WaveClass_C|GetWaveNumber (Utilities|Array|Get(acopy) (Variables|Default|GetAllWaves) _result)) _enemies_amount)
          (if (> (Variables|Default|GetCurrentWave) 0)
            (Utilities|FlowControl|Sequence
              (:then_0
                (if (LocalVariables|GetNextWaveType)
                  (Audio|PlaySound2D "/Game/Sound/SFX/UI/NewHardWave_Cue.NewHardWave_Cue" 1.0 1.0 0.0 0 0)
                  (CallFunction|OnBossWave)
                  (else
                    (Audio|PlaySound2D "/Game/Sound/SFX/UI/NewNormalWaveIncoming_Cue.NewNormalWaveIncoming_Cue" 1.0 1.0 0.0 0 0))))
              (:then_1
                (CallFunction|CheckMusicWave (LocalVariables|GetCurrentWaveType) (LocalVariables|GetNextWaveType))))))))))

(fn OnBossKill
  (Default|OnBossKill (CallFunction|GetFrontlinePlayerController)))

(fn RegisterFodderEnemy
  (params (Fodder :type BP%20Enemy%20Base%20Object%20Reference))
  (Utilities|Array|AddUnique (Variables|Default|GetActiveEnemies) Fodder))

(fn CheckMusicWave
  (params (PrevIsBoss :type Boolean) (NewIsBoss :type Boolean))
  (bind _gameinstancefrontline (CallFunction|GetFrontlineGameInstance))
  (Utilities|FlowControl|Sequence
    (:then_0
      (if (and PrevIsBoss (not NewIsBoss))
        (LocalVariables|SetMusicToPlay "/Game/Sound/Music/TSMusic_Castle.TSMusic_Castle")
        (elif (and (not PrevIsBoss) NewIsBoss)
          (LocalVariables|SetMusicToPlay "/Game/Sound/Music/Iván_Piccione_-_Scorcher_Theme_Cue.Iván_Piccione_-_Scorcher_Theme_Cue"))))
    (:then_1
      (Utilities|IsValid (LocalVariables|GetMusicToPlay)
        (:Is%20Valid
          (bind _musiccontroller (Variables|/Game/Blueprints/Managers/GI_Frontline.GI_Frontline_C|GetMusicController _gameinstancefrontline)
            (:then
              (Audio|Components|Audio|Stop _musiccontroller)
              (Audio|Components|Audio|SetSound _musiccontroller (LocalVariables|GetMusicToPlay))
              (Audio|Components|Audio|Play _musiccontroller 0.0))
            (:else
              (bind _returnvalue (Audio|CreateSound2D (LocalVariables|GetMusicToPlay) 1.0 1.0 0.0 0 true false))
              (bind _output_get (Variables|/Game/Blueprints/Managers/GI_Frontline.GI_Frontline_C|SetMusicController _gameinstancefrontline _returnvalue))
              (Audio|Components|Audio|Play _output_get 0.0)))
          (Variables|/Game/Blueprints/Managers/GI_Frontline.GI_Frontline_C|SetCurrentMusic _gameinstancefrontline (LocalVariables|GetMusicToPlay)))))))