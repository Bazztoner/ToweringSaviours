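; BP_SaveGame holds player progress stats, covering waves reached, enemy kills and the last hero used.
; It tracks global totals and bests alongside per-hero maps for wave reached, most kills and total kills, keyed by the Mage, Assassin and Demolisher heroes.
; ResetStats zeroes the global counters, writes zero for each hero in every map and clears the last hero used.
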(fn ResetStats
  (bind _heroenemiesmaxkilled (Variables|Default|GetHeroEnemiesMaxKilled))
  (bind _herowavereached (Variables|Default|GetHeroWaveReached))
  (bind _heroenemiestotalkilled (Variables|Default|GetHeroEnemiesTotalKilled))
  (Variables|Default|SetMaxWaveReached 0)
  (Variables|Default|SetMaxEnemiesKilled 0)
  (Variables|Default|SetEnemiesKilledTotal 0)
  (Utilities|Map|Add _heroenemiesmaxkilled "/Game/Blueprints/Characters/Frontline/Hero/BP_HeroMage.BP_HeroMage_C" 0)
  (Utilities|Map|Add _heroenemiesmaxkilled "/Game/Blueprints/Characters/Frontline/Hero/BP_HeroAssassin.BP_HeroAssassin_C" 0)
  (Utilities|Map|Add _heroenemiesmaxkilled "/Game/Blueprints/Characters/Frontline/Hero/BP_HeroDemolisher.BP_HeroDemolisher_C" 0)
  (Utilities|Map|Add _herowavereached "/Game/Blueprints/Characters/Frontline/Hero/BP_HeroMage.BP_HeroMage_C" 0)
  (Utilities|Map|Add _herowavereached "/Game/Blueprints/Characters/Frontline/Hero/BP_HeroAssassin.BP_HeroAssassin_C" 0)
  (Utilities|Map|Add _herowavereached "/Game/Blueprints/Characters/Frontline/Hero/BP_HeroDemolisher.BP_HeroDemolisher_C" 0)
  (Utilities|Map|Add _heroenemiestotalkilled "/Game/Blueprints/Characters/Frontline/Hero/BP_HeroMage.BP_HeroMage_C" 0)
  (Utilities|Map|Add _heroenemiestotalkilled "/Game/Blueprints/Characters/Frontline/Hero/BP_HeroAssassin.BP_HeroAssassin_C" 0)
  (Utilities|Map|Add _heroenemiestotalkilled "/Game/Blueprints/Characters/Frontline/Hero/BP_HeroDemolisher.BP_HeroDemolisher_C" 0)
  (Variables|Default|SetLastHeroUsed 0))