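; Wave data and progress tracker that picks objective and fodder enemy classes to spawn and decides when a wave is finished.
; Each pick rolls percentage chances key by key, taking the first success or falling back to a random key if no class is set.
; It records spawned objective enemies against the wave total and counts deaths.
; When kills reach that total, it clears the objective flag on valid listed enemies and reports completion.
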(event EventBeginPlay)

(event Collision|EventActorBeginOverlap
  (params (OtherActor :type Actor%20Object%20Reference)))

(event EventTick
  (params (DeltaSeconds :type Float%20%28single-precision%29)))

(fn ConstructionScript)

(fn GetEnemyObjective
  (bind _enemyobjectivedata (Variables|Default|GetEnemyObjectiveData))
  (bind _enemychance (Utilities|Struct|BreakSTRUCT_WaveData _enemyobjectivedata))
  (bind _keys (Utilities|Map|Keys _enemychance))
  (bind _array_element (Utilities|Array|ForEachLoopwithBreak _keys :!label _label)
    (:LoopBody
      (if (Math|Random|RandomBoolwithWeight (/ (Math|Conversions|ToFloat(Integer) (.Value (Utilities|Map|Find _enemychance _array_element))) 1e+02))
        (LocalVariables|SetEnemyToSpawn _array_element)
        (goto _label Break)))
    (:Completed
      (if (Utilities|IsValidClass (LocalVariables|GetEnemyToSpawn))
        (return (LocalVariables|GetEnemyToSpawn))
        (else
          (return (.OutItem (Utilities|Array|Random _keys))))))))

(fn AddEnemyObjective
  (params (SpawnedEnemy :type BP%20Enemy%20Base%20Object%20Reference%20%28by%20ref%29))
  (Utilities|Array|AddUnique (Variables|Default|GetEnemyList) SpawnedEnemy)
  (Math|Integer|IncrementInt (Variables|Default|GetEnemiesSpawned)))

(fn GetEnemyObjectiveAmount
  (bind _enemyobjectivedata (Variables|Default|GetEnemyObjectiveData))
  (bind _totalenemies (Utilities|Struct|BreakSTRUCT_WaveData _enemyobjectivedata))
  (return _totalenemies (< (Variables|Default|GetEnemiesSpawned) _totalenemies)))

(fn OnEnemyDeath
  (bind _result (Math|Integer|IncrementInt (Variables|Default|GetEnemiesKilled))
    (:%20%20
      (bind _output_get (Variables|Default|SetbWaveFinished (>= _result (.TotalEnemies (Utilities|Struct|BreakSTRUCT_WaveData (Variables|Default|GetEnemyObjectiveData))))))
      (if _output_get
        (for _array_element (Variables|Default|GetEnemyList)
          (Utilities|IsValid _array_element
            (:Is%20Valid
              (Variables|/Game/Blueprints/Characters/Frontline/Enemy/BP_EnemyBase.BP_EnemyBase_C|SetIsWaveObjective _array_element false))))
        (return _output_get)))))

(fn GetEnemiesinWave
  (return (.TotalEnemies (Utilities|Struct|BreakSTRUCT_WaveData (Variables|Default|GetEnemyObjectiveData)))))

(fn GetFodder
  (bind _fodderdata (Variables|Default|GetFodderData))
  (bind _enemychance (Utilities|Struct|BreakSTRUCT_WaveData _fodderdata))
  (bind _keys (Utilities|Map|Keys _enemychance))
  (bind _array_element (Utilities|Array|ForEachLoopwithBreak _keys :!label _label)
    (:LoopBody
      (if (Math|Random|RandomBoolwithWeight (/ (Math|Conversions|ToFloat(Integer) (.Value (Utilities|Map|Find _enemychance _array_element))) 1e+02))
        (LocalVariables|SetEnemyToSpawn _array_element)
        (goto _label Break)))
    (:Completed
      (if (Utilities|IsValidClass (LocalVariables|GetEnemyToSpawn))
        (return (LocalVariables|GetEnemyToSpawn))
        (else
          (return (.OutItem (Utilities|Array|Random _keys))))))))