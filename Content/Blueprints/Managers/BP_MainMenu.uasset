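; Main menu manager that shows the menu widget, sets Game and UI input with a visible cursor, and starts the menu theme on BeginPlay.
; The theme replaces any music controller on the Frontline game instance and persists across level transitions.
; It swaps the placed character-selection hero for one from the Heroes map, keyed by the save game's last-used hero, falling back to the instance's player character.
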(event EventBeginPlay
  (bind _gameinstancefrontline (CallFunction|GetFrontlineGameInstance))
  (bind _returnvalue (Game|GetPlayerController 0))
  (bind _gameinstancefrontline_2 (CallFunction|GetFrontlineGameInstance))
  (Utilities|FlowControl|Sequence
    (:then_0
      (bind _returnvalue_2 (UserInterface|CreateWidget "/Game/Blueprints/Widgets/CharacterSelection/WBP_MainMenu.WBP_MainMenu_C"))
      (UserInterface|Viewport|AddtoViewport _returnvalue_2 0)
      (Input|SetInputModeGameandUI _returnvalue _returnvalue_2 "LockAlways" false false)
      (Variables|/Script/Engine.PlayerController|SetbShowMouseCursor _returnvalue true)
      (bind _musiccontroller (Variables|/Game/Blueprints/Managers/GI_Frontline.GI_Frontline_C|GetMusicController _gameinstancefrontline)
        (:then
          (Audio|Components|Audio|Stop _musiccontroller)
          (Components|DestroyComponent _musiccontroller))
        (:else
          _))
      (bind _returnvalue_3 (Audio|CreateSound2D "/Game/Sound/Music/Towering_Saviour_-_Main_Menu_theme_Cue.Towering_Saviour_-_Main_Menu_theme_Cue" 1.0 1.0 0.0 0 true false))
      (bind _output_get (Variables|/Game/Blueprints/Managers/GI_Frontline.GI_Frontline_C|SetMusicController _gameinstancefrontline _returnvalue_3))
      (Audio|Components|Audio|Play _output_get 0.0))
    (:then_1
      (bind _returnvalue_4 (Actor|GetActorOfClass "/Game/Blueprints/Characters/CharacterSelection/BP_CharacterSelectionHeroBase.BP_CharacterSelectionHeroBase_C"))
      (Variables|Default|SetCurrentHero _returnvalue_4))
    (:then_2
      (bind _lastheroused (Variables|/Game/Blueprints/Managers/SaveGame/BP_SaveGame.BP_SaveGame_C|GetLastHeroUsed (Variables|/Game/Blueprints/Managers/GI_Frontline.GI_Frontline_C|GetSaveGame _gameinstancefrontline_2))
        (:then
          (Game|SpawnActorfromClass (.Value (Utilities|Map|Find (Variables|Default|GetHeroes) _lastheroused)) (Transformation|GetActorTransform (Variables|Default|GetCurrentHero)) "AlwaysSpawn" "MultiplyWithRoot" 0 0)
          (Actor|DestroyActor (Variables|Default|GetCurrentHero))
          (Variables|Default|SetCurrentHero 0))
        (:else
          (bind _herocharacterpicked (Default|GetPlayerCharacter _gameinstancefrontline_2))
          (Game|SpawnActorfromClass (.Value (Utilities|Map|Find (Variables|Default|GetHeroes) _herocharacterpicked)) (Transformation|GetActorTransform (Variables|Default|GetCurrentHero)) "AlwaysSpawn" "MultiplyWithRoot" 0 0)
          (Actor|DestroyActor (Variables|Default|GetCurrentHero))
          (Variables|Default|SetCurrentHero 0))))))

(fn ConstructionScript)