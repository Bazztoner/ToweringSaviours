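; Manager for the character selection screen, where the player cycles through playable heroes.
; After a brief load delay, it spawns every hero class at the CharSelectSpawn-tagged actor, shows only the first, and opens the selection widget in UI-only input.
; ChangeHeroSelected steps the index with wraparound by toggling visibility, and GetSelectedHero returns the current one.
; It also starts the main menu theme through the game instance, persisting across levels, unless already current.
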(event Custom|ChangeHeroSelected
  (params (Right :type Boolean))
  (CallFunction|ChangeHeroIndex Right))

(event EventBeginPlay
  (bind _gameinstancefrontline (CallFunction|GetFrontlineGameInstance))
  (bind _returnvalue (Game|GetPlayerController 0))
  (bind _allheroes (Variables|Default|GetAllHeroes))
  (Default|OnLoadStart _gameinstancefrontline)
  (Utilities|FlowControl|Delay 2.0)
  (Default|OnLoadEnd _gameinstancefrontline)
  (Utilities|FlowControl|Sequence
    (:then_0
      (bind _outactors (Actor|GetAllActorsOfClasswithTag "/Script/Engine.Actor" "CharSelectSpawn"))
      (bind _output_get (Variables|Default|SetHeroPos (Transformation|GetActorLocation (Utilities|Array|Get(acopy) _outactors)))))
    (:then_1
      (for _array_element (Variables|Default|GetHeroClasses)
        (bind _returnvalue_2 (Game|SpawnActorfromClass _array_element (Math|Transform|MakeTransform _output_get "0, 0, 0" "1.000000,1.000000,1.000000") "AlwaysSpawn" "OverrideRootScale" 0 0))
        (Rendering|SetActorHiddenInGame _returnvalue_2 true)
        (Utilities|Array|AddUnique (Variables|Default|GetAllHeroes) _returnvalue_2))
      (Rendering|SetActorHiddenInGame (Utilities|Array|Get(acopy) _allheroes) false)
      (Variables|Default|SetHeroAmount (Utilities|Array|Length _allheroes)))
    (:then_2
      (Variables|/Script/Engine.PlayerController|SetbShowMouseCursor _returnvalue true)
      (bind _returnvalue_3 (UserInterface|CreateWidget "/Game/Blueprints/Widgets/CharacterSelection/WBP_CharacterSelectionScreen.WBP_CharacterSelectionScreen_C" _returnvalue self))
      (UserInterface|Viewport|AddtoViewport _returnvalue_3 0)
      (Input|SetInputModeUIOnly (Game|GetPlayerController 0) _returnvalue_3 "LockAlways" false))
    (:then_3
      (CallFunction|SetMusic))))

(fn ConstructionScript)

(fn GetSelectedHero
  (return (Utilities|Array|Get(acopy) (Variables|Default|GetAllHeroes) (Variables|Default|GetHeroIndex))))

(fn ChangeHeroIndex
  (params (Right :type Boolean))
  (Utilities|FlowControl|Sequence
    (:then_0
      (Rendering|SetActorHiddenInGame (Utilities|Array|Get(acopy) (Variables|Default|GetAllHeroes) (Variables|Default|GetHeroIndex)) true))
    (:then_1
      (if Right
        (if (>= (+ (Variables|Default|GetHeroIndex) 1) (Variables|Default|GetHeroAmount))
          (Variables|Default|SetHeroIndex 0)
          (else
            (Math|Integer|IncrementInt (Variables|Default|GetHeroIndex))))
        (elif (> (Variables|Default|GetHeroIndex) 0)
          (Math|Integer|DecrementInt (Variables|Default|GetHeroIndex))
          (else
            (Variables|Default|SetHeroIndex (- (Variables|Default|GetHeroAmount) 1))))))
    (:then_2
      (Rendering|SetActorHiddenInGame (Utilities|Array|Get(acopy) (Variables|Default|GetAllHeroes) (Variables|Default|GetHeroIndex)) false))))

(fn SetMusic
  (bind _gameinstancefrontline (CallFunction|GetFrontlineGameInstance))
  (bind _musiccontroller (Variables|/Game/Blueprints/Managers/GI_Frontline.GI_Frontline_C|GetMusicController _gameinstancefrontline)
    (:then
      (if (not (== (Variables|/Game/Blueprints/Managers/GI_Frontline.GI_Frontline_C|GetCurrentMusic _gameinstancefrontline) "/Game/Sound/Music/Towering_Saviour_-_Main_Menu_theme_Cue.Towering_Saviour_-_Main_Menu_theme_Cue"))
        (Audio|Components|Audio|Stop _musiccontroller)
        (Components|DestroyComponent _musiccontroller)
        (bind _returnvalue (Audio|CreateSound2D "/Game/Sound/Music/Towering_Saviour_-_Main_Menu_theme_Cue.Towering_Saviour_-_Main_Menu_theme_Cue" 1.0 1.0 0.0 0 true false :!label _label))
        (bind _output_get (Variables|/Game/Blueprints/Managers/GI_Frontline.GI_Frontline_C|SetMusicController _gameinstancefrontline _returnvalue))
        (Audio|Components|Audio|Play _output_get 0.0)
        (Variables|/Game/Blueprints/Managers/GI_Frontline.GI_Frontline_C|SetCurrentMusic (CallFunction|GetFrontlineGameInstance) "/Game/Sound/Music/Towering_Saviour_-_Main_Menu_theme_Cue.Towering_Saviour_-_Main_Menu_theme_Cue")))
    (:else
      (goto _label))))