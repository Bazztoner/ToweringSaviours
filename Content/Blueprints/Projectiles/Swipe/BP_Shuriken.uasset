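; Spinning shuriken projectile that flies out, reverses like a boomerang and damages enemies it overlaps.
; A timer at half its lifetime negates horizontal velocity and zeroes vertical velocity before the parent BeginPlay runs its own logic.
; Each overlap with a BP_EnemyBase plays a hit sound and applies damage, with no destroy on hit here.
; Tick yaws the sprite at a constant rate.
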(event Custom|ReverseDirection
  (Variables|/Script/Engine.MovementComponent|SetVelocity (Variables|Default|GetProjectileMovement) (* (Variables|/Script/Engine.MovementComponent|GetVelocity (Variables|Default|GetProjectileMovement)) "-1.000000,-1.000000,0.000000")))

(event EventTick
  (params (DeltaSeconds :type Float%20%28single-precision%29))
  (Transformation|AddLocalRotation (Variables|Default|GetSprite) (Math|Rotator|MakeRotator 0.0 0.0 (* DeltaSeconds 2e+02)) false false))

(event Collision|EventActorBeginOverlap
  (params (OtherActor :type Actor%20Object%20Reference))
  (bind _asbp_enemy_base (Utilities|Casting|CastToBP_EnemyBase OtherActor))
  (Audio|PlaySoundatLocation (Variables|Default|GetHitSound) (Transformation|GetActorLocation _asbp_enemy_base) "0, 0, 0" 1.0 1.0 0.0 0 0 0 0)
  (Game|Damage|ApplyDamage _asbp_enemy_base (Variables|Default|GetDamage) 0 0))

(event EventBeginPlay
  (Utilities|Time|SetTimerbyEvent (delegate Custom|ReverseDirection) (/ (Variables|Default|GetLifetime) 2.0))
  (|CallParentFunction))

(fn ConstructionScript)