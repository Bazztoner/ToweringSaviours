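; BP_MagicBlast is a magic blast from the Swipe projectile set that stuns any BP_EnemyBase it overlaps for StunDuration.
; An OnActorAffected function applies damage and forward knockback with a separate Z force, using AffectedEnemies to hit each enemy only once.
; The event graph's call to that function is disconnected, so overlap in this graph only stuns.
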(event Collision|EventActorBeginOverlap
  (params (OtherActor :type Actor%20Object%20Reference))
  (bind _asbp_enemy_base (Utilities|Casting|CastToBP_EnemyBase OtherActor))
  (Default|OnStun _asbp_enemy_base (Variables|Default|GetStunDuration)))

(fn ConstructionScript)

(fn OnActorAffected
  (params (Object :type Object%20Object%20Reference))
  (bind _returnvalue (Transformation|GetActorForwardVector))
  (bind _knockbackforce (Variables|Default|GetKnockbackForce))
  (bind _returnvalue_2 (* _returnvalue _knockbackforce))
  (bind _asbp_enemy_base (Utilities|Casting|CastToBP_EnemyBase Object))
  (LocalVariables|SetEnemyAffected _asbp_enemy_base)
  (if (not (Utilities|Array|ContainsItem (Variables|Default|GetAffectedEnemies) (LocalVariables|GetEnemyAffected)))
    (Utilities|Array|AddUnique (Variables|Default|GetAffectedEnemies) (LocalVariables|GetEnemyAffected))
    (Default|ApplyKnockback (LocalVariables|GetEnemyAffected) (Math|Vector|MakeVector (.x _returnvalue_2) (.y _returnvalue_2) (Variables|Default|GetKnockbackZForce)))
    (Game|Damage|ApplyDamage (LocalVariables|GetEnemyAffected) (Variables|Default|GetDamage) 0 0)))