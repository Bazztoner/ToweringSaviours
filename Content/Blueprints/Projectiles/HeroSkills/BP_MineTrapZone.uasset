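; BP_MineTrapZone is a hero skill actor that scatters caltrop mines around its location.
; On BeginPlay it spawns a configurable number of BP_CaltropMine actors, passing each its damage, explosion radius and lifetime.
; Spawn points are random navigable locations within the spawn radius, keeping mines on the navmesh.
; An older random point-in-sphere helper, flattened to zero Z, remains but is unused.
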(event EventBeginPlay
  (for _index (range 1 (Variables|Default|GetCaltropAmount))
    (Game|SpawnActorfromClass "/Game/Blueprints/Projectiles/HeroSkills/BP_CaltropMine.BP_CaltropMine_C" (Math|Transform|MakeTransform (CallFunction|GetRandomSpawnPoint) "0, 0, 0" "1.000000,1.000000,1.000000") "AlwaysSpawn" "MultiplyWithRoot" 0 (Variables|Default|GetCaltropDamage) (Variables|Default|GetCaltropExplosionRadius) (Variables|Default|GetCaltropLifeTime) 0)))

(fn ConstructionScript)

(fn GetRandomPointinSphere
  (bind _returnvalue (Math|Random|RandomUnitVector))
  (bind _returnvalue_2 (Transformation|GetActorLocation))
  (bind _spawnradius (Variables|Default|GetSpawnRadius))
  (bind _returnvalue_3 (Math|Random|RandomFloatinRange 0.0 _spawnradius))
  (bind _returnvalue_4 (* _returnvalue _returnvalue_3))
  (bind _returnvalue_5 (+ _returnvalue_4 _returnvalue_2))
  (return (Math|Vector|MakeVector (.x _returnvalue_5) (.y _returnvalue_5) 0.0)))

(fn GetRandomSpawnPoint
  (bind _randomlocation (Class|NavigationSystemV1|GetRandomLocationinNavigableRadius (Transformation|GetActorLocation) (Variables|Default|GetSpawnRadius) 0 0))
  (return _randomlocation))