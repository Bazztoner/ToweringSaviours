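; BP_CaltropMine is a hero skill mine that damages nearby enemies when it explodes.
; After a one-tick delay at BeginPlay, a timeline moves it along its FlightPath spline without sweeping.
; It detonates on overlap with a BP_EnemyBase or when its lifetime timer expires.
; Explode spawns effects and sound, damages enemy pawns found by a sphere overlap, then destroys the actor.
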(event Custom|DelayedExplosion
  (CallFunction|Explode))

(event EventBeginPlay
  (Utilities|Time|SetTimerbyEvent (delegate Custom|DelayedExplosion) (Variables|Default|GetLifeTime))
  (Utilities|FlowControl|DelayUntilNextTick)
  (bind _alpha (Timeline|Timeline Play)
    (:Update
      (Transformation|SetActorLocation (Spline|GetLocationatTime (Variables|Default|GetFlightPath) _alpha "World" false) false false))))

(event Collision|EventActorBeginOverlap
  (params (OtherActor :type Actor%20Object%20Reference))
  (Utilities|Casting|CastToBP_EnemyBase OtherActor)
  (CallFunction|Explode))

(fn ConstructionScript)

(fn Explode
  (Utilities|FlowControl|Sequence
    (:then_0
      (Effects|SpawnEmitteratLocation "/Game/StarterContent/Particles/P_Explosion.P_Explosion" (Transformation|GetActorLocation) "0, 0, 0" "1.000000,1.000000,1.000000" true "AutoRelease")
      (Audio|SpawnSoundatLocation (Variables|Default|GetExplosionSound) (Transformation|GetActorLocation) "0, 0, 0" 1.0 1.0 0.0 0 0))
    (:then_1
      (bind (_outactors _returnvalue) (Collision|SphereOverlapActors (Transformation|GetActorLocation) (Variables|Default|GetExplosionRadius) (Utilities|Array|MakeArray "ObjectTypeQuery3") "/Game/Blueprints/Characters/Frontline/Enemy/BP_EnemyBase.BP_EnemyBase_C"))
      (if _returnvalue
        (for _array_element _outactors
          (Game|Damage|ApplyDamage _array_element (Variables|Default|GetDamage) 0 0))))
    (:then_2
      (Actor|DestroyActor))))