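; BP_FragGrenade is a hero skill grenade projectile that explodes on contact with an enemy or on reaching its target position.
; Each tick it spins its mesh and checks 2D distance to the target, detonating within a small threshold.
; The explosion plays effects and sound, then sphere-overlaps enemy pawns to apply outward knockback with slight lift plus damage credited to the first player controller, then destroys itself.
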(event Collision|EventActorBeginOverlap
  (params (OtherActor :type Actor%20Object%20Reference))
  (Utilities|Casting|CastToBP_EnemyBase OtherActor)
  (CallFunction|Explode))

(event EventTick
  (params (DeltaSeconds :type Float%20%28single-precision%29))
  (CallFunction|RotateMesh DeltaSeconds)
  (CallFunction|CheckDistancetoTarget))

(event EventBeginPlay
  (Audio|PlaySoundatLocation (Variables|Default|GetLaunchSound) (Transformation|GetActorLocation) "0, 0, 0" 1.0 1.0 0.0 0 0 0 0))

(fn ConstructionScript)

(fn RotateMesh
  (params (DeltaTime :type Float%20%28double-precision%29))
  (bind _returnvalue (* DeltaTime 185.0))
  (Transformation|AddLocalRotation (Variables|Default|GetStaticMesh) (Math|Rotator|MakeRotator _returnvalue _returnvalue _returnvalue) false false))

(fn CheckDistancetoTarget
  (if (<= (Math|Vector|Distance2D(Vector) (Math|Conversions|ToVector2D(Vector) (Transformation|GetActorLocation)) (Math|Conversions|ToVector2D(Vector) (Variables|Default|GetTargetPos))) 1e+01)
    (CallFunction|Explode)))

(fn Explode
  (bind _returnvalue (Game|GetPlayerController 0))
  (Utilities|FlowControl|Sequence
    (:then_0
      (Effects|SpawnEmitteratLocation "/Game/StarterContent/Particles/P_Explosion.P_Explosion" (Transformation|GetActorLocation) "0, 0, 0" "1.000000,1.000000,1.000000" true "AutoRelease")
      (Audio|SpawnSound2D (Variables|Default|GetExplosionSound) 1.0 1.0 0.0 0))
    (:then_1
      (bind (_outactors _returnvalue_2) (Collision|SphereOverlapActors (Transformation|GetActorLocation) (Variables|Default|GetExplosionRadius) (Utilities|Array|MakeArray "ObjectTypeQuery3") "/Game/Blueprints/Characters/Frontline/Enemy/BP_EnemyBase.BP_EnemyBase_C"))
      (if _returnvalue_2
        (for _array_element _outactors
          (bind _asbp_enemy_base (Utilities|Casting|CastToBP_EnemyBase _array_element))
          (Default|ApplyKnockback _asbp_enemy_base (Math|Vector|MakeVector (.x (* (Class|KismetMathLibrary|VectorNormal2D (- (Transformation|GetActorLocation _asbp_enemy_base) (Transformation|GetActorLocation)) 0.0001) (Variables|Default|GetKickbackForce))) (.y (* (Class|KismetMathLibrary|VectorNormal2D (- (Transformation|GetActorLocation _asbp_enemy_base) (Transformation|GetActorLocation)) 0.0001) (Variables|Default|GetKickbackForce))) 15.0))
          (Game|Damage|ApplyDamage _array_element (Variables|Default|GetDamage) _returnvalue _returnvalue))))
    (:then_2
      (Actor|DestroyActor))))