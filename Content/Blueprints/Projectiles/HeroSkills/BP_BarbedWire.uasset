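; BP_BarbedWire is a hero skill hazard that slows and damages enemies inside it for a limited lifetime.
; On spawn it traces downward to match the rotation of the lane beneath, plays its sound and starts timers for self-destruction and damage ticks.
; Overlap events toggle the slow on enemies and maintain the list that each tick damages, scaling damage per second by tick duration.
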(event Custom|ApplyDamage
  (for _array_element (Variables|Default|GetEnemyList)
    (Utilities|IsValid _array_element
      (:Is%20Valid
        (Game|Damage|ApplyDamage _array_element (* (Variables|Default|GetDamagePerSecond) (Variables|Default|GetTickDuration)) 0 0)))))

(event Custom|DelayedDestroy
  (Actor|DestroyActor))

(event EventBeginPlay
  (Utilities|FlowControl|Sequence
    (:then_0
      (CallFunction|SetRotationbyLane))
    (:then_1
      (Audio|SpawnSoundAttached (Variables|Default|GetSkillSound) (Variables|Default|GetDefaultSceneRoot) "None" (Transformation|GetActorLocation) "0, 0, 0" "KeepRelativeOffset" true 1.0 1.0 0.0 0 0))
    (:then_2
      (Utilities|Time|SetTimerbyEvent (delegate Custom|DelayedDestroy) (Variables|Default|GetLifeTime)))
    (:then_3
      (Utilities|Time|SetTimerbyEvent (delegate Custom|ApplyDamage) (Variables|Default|GetTickDuration) true))))

(event Collision|EventActorEndOverlap
  (params (OtherActor :type Actor%20Object%20Reference))
  (CallFunction|CheckActorSlow false OtherActor)
  (bind _asbp_enemy_base (Utilities|Casting|CastToBP_EnemyBase OtherActor))
  (Utilities|Array|RemoveItem (Variables|Default|GetEnemyList) _asbp_enemy_base))

(event Collision|EventActorBeginOverlap
  (params (OtherActor :type Actor%20Object%20Reference))
  (CallFunction|CheckActorSlow true OtherActor)
  (bind _asbp_enemy_base (Utilities|Casting|CastToBP_EnemyBase OtherActor))
  (Utilities|Array|AddUnique (Variables|Default|GetEnemyList) _asbp_enemy_base))

(fn ConstructionScript)

(fn CheckActorSlow
  (params (Slow :type Boolean) (Actor :type Actor%20Object%20Reference))
  (bind _asbp_enemy_base (Utilities|Casting|CastToBP_EnemyBase Actor))
  (Default|OnSlowApplied _asbp_enemy_base (Variables|Default|GetSlowMultiplier) Slow))

(fn SetRotationbyLane
  (bind _returnvalue (Transformation|GetActorLocation))
  (bind (_x _y _z) (Math|Vector|BreakVector _returnvalue))
  (bind (_outhit _returnvalue_2) (Collision|LineTraceByChannel _returnvalue (Math|Vector|MakeVector _x _y (- _z 5e+03)) "TraceTypeQuery1" false 0 "None"))
  (if _returnvalue_2
    (if (Actor|ActorHasTag (.HitActor (Collision|BreakHitResult _outhit)) "LevelLane")
      (Transformation|SetActorRotation (Transformation|GetActorRotation (.HitActor (Collision|BreakHitResult _outhit)))))))