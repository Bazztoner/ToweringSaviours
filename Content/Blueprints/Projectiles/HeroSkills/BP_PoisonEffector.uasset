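; Poison status-effect component that slows its owning BP_EnemyBase and damages it over time.
; BeginPlay caches the enemy owner, applies the slow and uses the component tick interval as the damage cadence.
; Each tick applies damage and accumulates elapsed time; once the effect duration is reached, it clears the slow and destroys itself.
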(event EventBeginPlay
  (bind _asbp_enemy_base (Utilities|Casting|CastToBP_EnemyBase (Components|GetOwner)))
  (Variables|Default|SetEnemyOwner _asbp_enemy_base)
  (Class|ActorComponent|SetComponentTickIntervalandCooldown (Variables|Default|GetTickDuration))
  (bind _enemyowner (Variables|Default|GetEnemyOwner)
    (:then
      (Default|ApplySlow _enemyowner (Variables|Default|GetSlowAmount) true))
    (:else)))

(event EventTick
  (params (DeltaSeconds :type Float%20%28single-precision%29))
  (bind _enemyowner (Variables|Default|GetEnemyOwner)
    (:then
      (Game|Damage|ApplyDamage _enemyowner (Variables|Default|GetDamagePerTick) 0 0)
      (bind _output_get (Variables|Default|SetTimeElapsed (+ (Variables|Default|GetTimeElapsed) DeltaSeconds)))
      (if (>= _output_get (Variables|Default|GetEffectorDuration))
        (Default|ApplySlow (Variables|Default|GetEnemyOwner) 0.0 false)
        (Components|DestroyComponent)))
    (:else)))