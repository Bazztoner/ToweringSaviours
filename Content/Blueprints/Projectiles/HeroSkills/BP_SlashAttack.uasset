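; BP_SlashAttack is a short-lived hero skill actor that sweeps a melee slash hitbox through an arc.
; On spawn it hides its sprite, plays a start sound and turns the hitbox pivot back by half the attack angle.
; Tick rotates the pivot at a constant rate, covering the full angle over its lifespan.
; Overlapped BP_EnemyBase actors take damage and spawn a hit sound and pooled particle.
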(event EventBeginPlay
  (Sprite|SetSpriteColor (Variables|Default|GetPaperSprite) "(R=1.000000,G=1.000000,B=1.000000,A=0.000000)")
  (Actor|SetLifeSpan (Variables|Default|GetLifeSpan))
  (Audio|SpawnSoundatLocation (Variables|Default|GetStartSound) (Transformation|GetActorLocation) "0, 0, 0" 1.0 1.0 0.0 0 0)
  (Transformation|SetRelativeRotation (Variables|Default|GetAttackHitboxPivot) (Math|Rotator|MakeRotator 0.0 0.0 (* (/ (Variables|Default|GetAttackAngle) 2.0) -1.0)) false false))

(event Collision|EventActorBeginOverlap
  (params (OtherActor :type Actor%20Object%20Reference))
  (bind _asbp_enemy_base (Utilities|Casting|CastToBP_EnemyBase OtherActor))
  (Game|Damage|ApplyDamage _asbp_enemy_base (Variables|Default|GetDamage) 0 0)
  (Utilities|IsValid _asbp_enemy_base
    (:Is%20Valid
      (Audio|SpawnSoundatLocation (Variables|Default|GetHitSound) (Transformation|GetActorLocation _asbp_enemy_base) "0, 0, 0" 1.0 1.0 0.0 0 0)
      (Effects|SpawnEmitteratLocation (Variables|Default|GetHitParticle) (Transformation|GetActorLocation _asbp_enemy_base) "0, 0, 0" "1.000000,1.000000,1.000000" true "AutoRelease"))))

(event EventTick
  (params (DeltaSeconds :type Float%20%28single-precision%29))
  (bind _output_get (Variables|Default|SetTimeElapsed (+ DeltaSeconds (Variables|Default|GetTimeElapsed))))
  (CallFunction|RotateAttack DeltaSeconds))

(fn ConstructionScript)

(fn RotateAttack
  (params (Tick :type Float%20%28double-precision%29))
  (Transformation|AddRelativeRotation (Variables|Default|GetAttackHitboxPivot) (Math|Rotator|MakeRotator 0.0 0.0 (/ (* Tick (Variables|Default|GetAttackAngle)) (Variables|Default|GetLifeSpan))) false false))