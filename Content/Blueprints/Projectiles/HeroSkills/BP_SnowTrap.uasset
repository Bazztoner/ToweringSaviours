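; BP_SnowTrap is a hero skill trap actor that slows enemies inside it for a limited lifetime.
; On spawn it plays an attached sound and grows its mesh via a timeline driving scale.
; A timer set to lifetime minus timeline length reverses that animation, and the actor destroys itself when the shrink finishes.
; Overlap begin and end toggle the slow on BP_EnemyBase actors through CheckActorSlow.
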(event Custom|DelayedDestroy
  (bind (_direction _sizetrack) (Timeline|GrowAnimation ReverseFromEnd)
    (:Update
      (Transformation|SetWorldScale3D (Variables|Default|GetMesh) _sizetrack))
    (:Finished
      (switch Utilities|FlowControl|Switch|SwitchonETimelineDirection _direction
        (:Backward
          (Actor|DestroyActor))))))

(event EventBeginPlay
  (Utilities|FlowControl|Sequence
    (:then_0
      (Audio|SpawnSoundAttached (Variables|Default|GetSkillSound) (Variables|Default|GetDefaultSceneRoot) "None" (Transformation|GetActorLocation) "0, 0, 0" "KeepRelativeOffset" true 1.0 1.0 0.0 0 0))
    (:then_1
      (Utilities|Time|SetTimerbyEvent (delegate Custom|DelayedDestroy) (- (Variables|Default|GetLifeTime) (Components|Timeline|GetTimelineLength (Variables|Default|GetGrowAnimation)))))
    (:then_2
      (bind (_direction _sizetrack) (Timeline|GrowAnimation PlayFromStart)
        (:Update
          (Transformation|SetWorldScale3D (Variables|Default|GetMesh) _sizetrack))
        (:Finished
          (switch Utilities|FlowControl|Switch|SwitchonETimelineDirection _direction
            (:Backward
              (Actor|DestroyActor))))))))

(event Collision|EventActorBeginOverlap
  (params (OtherActor :type Actor%20Object%20Reference))
  (CallFunction|CheckActorSlow true OtherActor))

(event Collision|EventActorEndOverlap
  (params (OtherActor :type Actor%20Object%20Reference))
  (CallFunction|CheckActorSlow false OtherActor))

(fn ConstructionScript)

(fn CheckActorSlow
  (params (Slow :type Boolean) (Actor :type Actor%20Object%20Reference))
  (bind _asbp_enemy_base (Utilities|Casting|CastToBP_EnemyBase Actor))
  (Default|OnSlowApplied _asbp_enemy_base (Variables|Default|GetSlowMultiplier) Slow))