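; BP_PoisonDagger is a hero skill projectile that poisons the enemy it hits.
; It sets its life span on BeginPlay and ignores overlaps with anything other than BP_EnemyBase.
; On an enemy overlap it plays a hit sound, adds a BP_PoisonEffector carrying slow and damage-over-time settings, then destroys itself.
; Damage per tick is derived from damage per second and tick duration.
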(event EventBeginPlay
  (Actor|SetLifeSpan (Variables|Default|GetLifeTime)))

(event Collision|EventActorBeginOverlap
  (params (OtherActor :type Actor%20Object%20Reference))
  (bind _tickduration (Variables|Default|GetTickDuration))
  (bind _asbp_enemy_base (Utilities|Casting|CastToBP_EnemyBase OtherActor))
  (Audio|PlaySoundatLocation (Variables|Default|GetHitSound) (Transformation|GetActorLocation _asbp_enemy_base) "0, 0, 0" 1.0 1.0 0.0 0 0 0 0)
  (Game|AddComponentbyClass _asbp_enemy_base "/Game/Blueprints/Projectiles/HeroSkills/BP_PoisonEffector.BP_PoisonEffector_C" (Variables|Default|GetSlowAmount) (* (Variables|Default|GetDamagePerSecond) _tickduration) _tickduration (Variables|Default|GetEffectorDuration))
  (Actor|DestroyActor))

(fn ConstructionScript)