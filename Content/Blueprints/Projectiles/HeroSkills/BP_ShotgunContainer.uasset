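; Shotgun hero-skill container that bursts into a horizontal fan of pellet projectiles when it begins play.
; It requires a BP_PlayerController owner, passed to each pellet as owner, with that controller's character as instigator.
; CreatePellets rotates the negated actor forward vector around world Z in even steps, starting at minus half of HalfAngle.
; Total Damage is divided evenly among the pellets.
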(event EventBeginPlay
  (bind _asbp_player_controller (Utilities|Casting|CastToBP_PlayerController (Components|GetOwner)))
  (Variables|Default|SetPlayerController _asbp_player_controller)
  (CallFunction|CreatePellets))

(fn ConstructionScript)

(fn CreatePellets
  (LocalVariables|SetAngleIncrement (/ (Variables|Default|GetHalfAngle) (Variables|Default|GetPellets)))
  (for _index (range 0 (- (Variables|Default|GetPellets) 1))
    (Game|SpawnActorfromClass (Variables|Default|GetProjectileClass) (Math|Transform|MakeTransform "0, 0, 0" (Math|Conversions|RotationFromXVector (Math|Vector|RotateVectorAroundAxis (Math|Vector|NegateVector (Transformation|GetActorForwardVector)) (+ (* (Variables|Default|GetHalfAngle) -0.5) (* _index (LocalVariables|GetAngleIncrement))) "0.000000,0.000000,1.000000")) "1.000000,1.000000,1.000000") "AlwaysSpawn" "MultiplyWithRoot" (Variables|Default|GetPlayerController) (/ (Variables|Default|GetDamage) (Variables|Default|GetPellets)) (Variables|/Game/Blueprints/Player/BP_PlayerController.BP_PlayerController_C|GetPlayerCharacter (Variables|Default|GetPlayerController)))))