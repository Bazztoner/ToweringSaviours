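; Flame well hero skill actor that deals periodic area damage to enemies for a limited lifetime, with an attached sound.
; Overlap events maintain a list of BP_EnemyBase actors, which a looping timer damages by damage-per-second scaled to the tick interval.
; A timeline scales the FlameWall in on spawn.
; A second timer, offset by the timeline's length, reverses that animation near the end of life, and the actor destroys itself when it finishes.
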(event Custom|ApplyDamage
  (for _array_element (Variables|Default|GetEnemyList)
    (Utilities|IsValid _array_element
      (:Is%20Valid
        (Game|Damage|ApplyDamage _array_element (* (Variables|Default|GetDamagePerSecond) (Variables|Default|GetTickDuration)) 0 0)))))

(event Custom|DelayedDestruction
  (bind (_direction _size) (Timeline|SpawnAnimation ReverseFromEnd)
    (:Update
      (Transformation|SetWorldScale3D (Variables|Default|GetFlameWall) _size))
    (:Finished
      (switch Utilities|FlowControl|Switch|SwitchonETimelineDirection _direction
        (:Backward
          (Actor|DestroyActor))))))

(event EventBeginPlay
  (Utilities|FlowControl|Sequence
    (:then_0
      (Utilities|Time|SetTimerbyEvent (delegate Custom|ApplyDamage) (Variables|Default|GetTickDuration) true)
      (Audio|SpawnSoundAttached (Variables|Default|GetSkillSound) (Variables|Default|GetDefaultSceneRoot) "None" (Transformation|GetActorLocation) "0, 0, 0" "KeepRelativeOffset" true 1.0 1.0 0.0 0 0))
    (:then_1
      (Utilities|Time|SetTimerbyEvent (delegate Custom|DelayedDestruction) (- (Variables|Default|GetLifeTime) (Components|Timeline|GetTimelineLength (Variables|Default|GetSpawnAnimation))))
      (bind (_direction _size) (Timeline|SpawnAnimation PlayFromStart)
        (:Update
          (Transformation|SetWorldScale3D (Variables|Default|GetFlameWall) _size))
        (:Finished
          (switch Utilities|FlowControl|Switch|SwitchonETimelineDirection _direction
            (:Backward
              (Actor|DestroyActor))))))))

(event Collision|EventActorBeginOverlap
  (params (OtherActor :type Actor%20Object%20Reference))
  (Utilities|IsValid OtherActor
    (:Is%20Valid
      (bind _asbp_enemy_base (Utilities|Casting|CastToBP_EnemyBase OtherActor))
      (Utilities|Array|AddUnique (Variables|Default|GetEnemyList) _asbp_enemy_base))))

(event Collision|EventActorEndOverlap
  (params (OtherActor :type Actor%20Object%20Reference))
  (Utilities|IsValid OtherActor
    (:Is%20Valid
      (bind _asbp_enemy_base (Utilities|Casting|CastToBP_EnemyBase OtherActor))
      (Utilities|Array|RemoveItem (Variables|Default|GetEnemyList) _asbp_enemy_base))))

(fn ConstructionScript)