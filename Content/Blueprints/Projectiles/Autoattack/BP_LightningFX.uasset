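; Lightning effect actor for an autoattack projectile that moves a Sphere component between two world positions.
; Each tick it lerps the sphere from start to end by elapsed time over a fifth of a second, with the alpha left unclamped.
; SetPositions restarts the travel, and SetNextTarget chains a new hop from the previous end point.
; The nodes that orient the sphere along its path are disconnected and never run.
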(event EventTick
  (params (DeltaSeconds :type Float%20%28single-precision%29))
  (Transformation|SetWorldLocation (Variables|Default|GetSphere) (Math|Vector|Lerp(Vector) (Variables|Default|GetStartPos) (Variables|Default|GetEndPos) (/ (Variables|Default|GetCurrentTime) 0.2)) false false)
  (Variables|Default|SetCurrentTime (+ DeltaSeconds (Variables|Default|GetCurrentTime))))

(fn ConstructionScript)

(fn SetPositions
  (params (Start :type Vector) (End :type Vector))
  (Variables|Default|SetStartPos Start)
  (Variables|Default|SetEndPos End)
  (Variables|Default|SetCurrentTime 0.0))

(fn SetNextTarget
  (params (NextTargetPos :type Vector))
  (CallFunction|SetPositions (Variables|Default|GetEndPos) NextTargetPos))