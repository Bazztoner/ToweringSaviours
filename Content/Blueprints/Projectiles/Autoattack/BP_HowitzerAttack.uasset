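; BP_HowitzerAttack is an autoattack projectile that creates an area explosion on its enemy target.
; On BeginPlay it teleports to the target, fires OnEnemyHit, scales ExplosionFX through the RadialGrow timeline, then destroys itself.
; Overlapping enemies are damaged once each, tracked in EnemiesHit.
; CheckEnemyHit computes FinalDamage with a bonus for the main target, but ApplyDamage passes only SplashDamage.
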(event EventBeginPlay
  (bind _enemytarget (Variables|Default|GetEnemyTarget))
  (bind _returnvalue (Transformation|GetActorLocation _enemytarget))
  (Transformation|Teleport _returnvalue "0, 0, 0")
  (CallFunction|OnEnemyHit _returnvalue)
  (bind _size (Timeline|RadialGrow PlayFromStart)
    (:Update
      (Transformation|SetWorldScale3D (Variables|Default|GetExplosionFX) _size))
    (:Finished
      (Actor|DestroyActor))))

(event Collision|EventActorBeginOverlap
  (params (OtherActor :type Actor%20Object%20Reference))
  (bind _asbp_enemy_base (Utilities|Casting|CastToBP_EnemyBase OtherActor))
  (if (not (Utilities|Array|ContainsItem (Variables|Default|GetEnemiesHit) _asbp_enemy_base))
    (CallFunction|CheckEnemyHit _asbp_enemy_base)))

(fn ConstructionScript
  (|CallParentFunction))

(fn OnEnemyHit
  (params (HitLocation :type Vector :default "0, 0, 0"))
  (|CallParentFunction HitLocation))

(fn CheckEnemyHit
  (params (Enemy :type BP%20Enemy%20Base%20Object%20Reference%20%28by%20ref%29))
  (bind _returnvalue (Game|GetPlayerController 0))
  (Utilities|FlowControl|Sequence
    (:then_0
      (Utilities|Array|AddUnique (Variables|Default|GetEnemiesHit) Enemy)
      (if (== Enemy (Variables|Default|GetEnemyTarget))
        (LocalVariables|SetFinalDamage (+ (Variables|Default|GetSplashDamage) (Variables|Default|GetDamage)))
        (else
          (LocalVariables|SetFinalDamage (Variables|Default|GetSplashDamage)))))
    (:then_1
      (Game|Damage|ApplyDamage Enemy (Variables|Default|GetSplashDamage) _returnvalue _returnvalue))))