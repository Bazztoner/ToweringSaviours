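; BP_DaggerAttack is a dagger auto-attack projectile that homes in on an enemy and damages it on contact.
; On BeginPlay it homes on the EnemyTarget's capsule component, or disables homing when no valid target exists.
; Overlapping any BP_EnemyBase calls OnEnemyHit with the enemy's location, applies Damage and destroys the projectile, while other actors are ignored.
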(event EventBeginPlay
  (Utilities|IsValid (Variables|Default|GetEnemyTarget)
    (:Is%20Valid
      (Variables|/Script/Engine.ProjectileMovementComponent|SetHomingTargetComponent (Variables|Default|GetProjectileMovement) (Variables|/Script/Engine.Character|GetCapsuleComponent (Variables|Default|GetEnemyTarget))))
    (:Is%20Not%20Valid
      (Variables|/Script/Engine.ProjectileMovementComponent|SetbIsHomingProjectile (Variables|Default|GetProjectileMovement) false))))

(event Collision|EventActorBeginOverlap
  (params (OtherActor :type Actor%20Object%20Reference))
  (bind _asbp_enemy_base (Utilities|Casting|CastToBP_EnemyBase OtherActor))
  (CallFunction|OnEnemyHit (Transformation|GetActorLocation _asbp_enemy_base))
  (Game|Damage|ApplyDamage _asbp_enemy_base (Variables|Default|GetDamage) 0 0)
  (Actor|DestroyActor))

(event EventTick
  (params (DeltaSeconds :type Float%20%28single-precision%29)))

(fn ConstructionScript)